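; Multiplayer VR player state that holds a player's personal state and shows it on a body-attached UI actor.
; On standalone, or on a remote with a valid player controller, BeginPlay binds to the BP_SocketIO user-data response and stores it through SendUserData.
; PersonalState's RepNotify updates the BM_PersonalState actor.
; SpawnPersonalStateUI creates that actor if missing and attaches it to the controlled BP_GateCharacter_VR's body.
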(event `self.ReceiveBeginPlay`
  (if (not (`KismetSystemLibrary.IsStandalone`))
    (`/Engine/EditorBlueprintResources/ActorMacros.Switch Has Authority`
      (:`Remote`
        (`/Engine/EditorBlueprintResources/StandardMacros.IsValid` (`self.GetPlayerController`)
          (:`Is Valid`
            _)))))
  (bind _returnvalue (`GameplayStatics.GetActorOfClass` "/Game/Multiplayer/BP_SocketIO.BP_SocketIO_C"))
  (`/Engine/EditorBlueprintResources/StandardMacros.IsValid` _returnvalue
    (:`Is Valid`
      (add `/Game/Multiplayer/BP_SocketIO.OnResponseUserData` _returnvalue (delegate `OnResponseUserData`)))))

(event `OnResponseUserData`
  (params (State :type "/Game/XHUD/Profile/FPlayer_NameTag Structure"))
  (`self.SendUserData` State))

(event `SendUserData`
  (params (State :type "/Game/XHUD/Profile/FPlayer_NameTag Structure"))
  (set `self.PersonalState` State))

(fn `OnRep_PersonalState`
  (bind _personalstateui (`self.PersonalStateUI`)
    (:`then`
      (`/Game/XHUD/Profile/BM_PersonalState.Update State` _personalstateui (`self.PersonalState`)))
    (:`else`)))

(fn `SpawnPersonalStateUI`
  (params (Owner :type "PlayerController Object Reference"))
  (`self.PersonalStateUI`
    (:`then`
      _)
    (:`else`
      (bind _returnvalue (`|SpawnActorFromClass` "/Game/XHUD/Profile/BM_PersonalState.BM_PersonalState_C" (`KismetMathLibrary.MakeTransform` (0.0 0.0 0.0)) "AlwaysSpawn" "OverrideRootScale" (`local.Owner`) null))
      (set `self.PersonalStateUI` _returnvalue)))
  (bind _asbp_gate_character_vr (cast `/Game/Multiplayer/Characters/FBIK/BP_GateCharacter_VR` (`Controller.K2_GetPawn` (`local.Owner`))))
  (`/Game/XHUD/Profile/BM_PersonalState.SetAttachTo` (`self.PersonalStateUI`) (`/Game/Multiplayer/Characters/FBIK/BP_GateCharacter_VR.Body` _asbp_gate_character_vr)))

(fn `UserConstructionScript`)