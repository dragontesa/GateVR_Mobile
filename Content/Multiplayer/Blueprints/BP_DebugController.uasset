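; Debug controller for multiplayer that assigns a random numeric string as the gate instance's UserID on BeginPlay, then calls the parent BeginPlay.
; An unconnected chain, which never runs, would set a high-quality music, game-streaming audio profile on the gate instance's RTC engine.
; That dead chain would then reapply the Pig King voice changer preset in a one-second Delay loop.
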(event `self.ReceiveBeginPlay`
  (set `/Game/Multiplayer/Blueprints/BP_GateGameInstance.UserID` (`KismetStringLibrary.Conv_IntToString` (`KismetMathLibrary.RandomInteger` 100000)) (`/Game/Multiplayer/Blueprints/GateVRFunctionLibrary.GetGateInstance`))
  (`parent.ReceiveBeginPlay`))

(fn `UserConstructionScript`
  (`parent.UserConstructionScript`))