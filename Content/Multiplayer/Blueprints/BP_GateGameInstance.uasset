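; Game instance for the multiplayer Gate game, holding session state, player settings and voice chat.
; Host setup reports through SocketIO, while player and match joins open hard-coded server IPs; GameLift paths are mostly disabled or unreachable.
; Agora RTC provides voice with mute, effects, volume indication and Oculus device selection, and is released before level changes and shutdown; spatial audio init is unwired.
; Settings persist through a save slot, with a random character when none exists.
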(event `self.ReceiveShutdown`
  ;[1 1 1] Shut Down
  (`self.ReleaseVoice`))

(event `self.HandleNetworkError`
  (params (FailureType :type "ENetworkFailure Enum" :default "NetDriverAlreadyExists") (bIsServer :type Boolean))
  ;[1 1 1] Handle Network Errors
  (`self.DisplayErrorMessage` (`self.NetErrorToString` FailureType)))

(event `self.HandleTravelError`
  (params (FailureType :type "ETravelFailure Enum" :default "NoLevel"))
  ;[1 1 1] Handle Travel Errors
  (`self.DisplayErrorMessage` (`self.TravelErrorToString` FailureType)))

(event `DestroySessionCaller`
  (params (PlayerController :type "PlayerController Object Reference"))
  ;[1 1 1] Destroy Session when called
  (`DestroySessionCallbackProxy.DestroySession` PlayerController))

(event `ExitGame`
  ;[1 1 1] Exit Game
  (`PlayerCameraManager.StartCameraFade` :`self` (`GameplayStatics.GetPlayerCameraManager` 0) :`ToAlpha` 1.0 :`Duration` 1.5 :`bHoldWhenFinished` true)
  (`KismetSystemLibrary.Delay` 2.0)
  (`KismetSystemLibrary.QuitGame` (`GameplayStatics.GetPlayerController` 0) "Quit"))

(event `Disconnect`
  (params (PlayerController :type "PlayerController Object Reference"))
  (`DestroySessionCallbackProxy.DestroySession` PlayerController
    (:`OnSuccess`
      (bind (_gategameliftref _gategameliftref_2) (`self.GateGameLiftRef` :!enabledstate Disabled)
        (:`then`
          (`Actor.K2_DestroyActor` _gategameliftref_2 :!enabledstate Disabled))
        (:`else`
          _))
      (`self.OpenLobby`))))

(event `JoinSession`
  (params (Adress :type String))
  ;[1 1 1] Join Session
  (`GameplayStatics.OpenLevel` (`KismetStringLibrary.Conv_StringToName` Adress)))

(event `OpenLevel`
  (params (Level :type Name))
  ;[1 1 1] OpenLevel With Camera Fade
  (`self.ReleaseVoice`)
  (`/Game/Multiplayer/Blueprints/BP_GatePlayerController.FadeIn` (`/Game/Multiplayer/Blueprints/GateVRFunctionLibrary.GetGateController`))
  (`self.OnLevelUnload`)
  (`KismetSystemLibrary.Delay` 3.0)
  (`GameplayStatics.OpenLevel` Level))

(fn `BindEventOnCreateGameSession`
  (`self.GateGameLiftRef` :!enabledstate Disabled
    (:`then`
      (if (`self.In Matching Game` :!enabledstate Disabled)
        (bind _asbp_socket_io_random_chat (cast `` (`/Game/Multiplayer/Blueprints/BP_GatePlayerController.SocketIoRef` (`/Game/Multiplayer/Blueprints/GateVRFunctionLibrary.GetGateController` :!enabledstate Disabled) :!enabledstate Disabled) :!enabledstate Disabled))
        (add `self.OnCreateGameSessionSuccess` (`.GateGameLiftRef` (`self.GateGameLiftRef` :!enabledstate Disabled)) (`|CreateDelegate` _asbp_socket_io_random_chat :!event `ue-matching-response-game-session`) :!enabledstate Disabled)
        (else
          (add `self.OnCreateGameSessionSuccess` (`.GateGameLiftRef` (`self.GateGameLiftRef` :!enabledstate Disabled)) (`|CreateDelegate` (`/Game/Multiplayer/Blueprints/BP_GatePlayerController.SocketIoRef` (`/Game/Multiplayer/Blueprints/GateVRFunctionLibrary.GetGateController` :!enabledstate Disabled) :!enabledstate Disabled) :!event `Send_Game_FleetID`) :!enabledstate Disabled))))
    (:`else`)))

(fn `CharacterSelect`
  (bind _characters (`self.Characters`))
  (setmembers `/Game/Multiplayer/Blueprints/FPlayerInfo` :`StructRef` (`self.PlayerSettings`) :`Character` (`|GetArrayItem` _characters (`KismetMathLibrary.RandomInteger` (`KismetArrayLibrary.Array_Length` _characters)))))

(fn `CheckSaveGame`
  (bind _returnvalue (`GameplayStatics.DoesSaveGameExist` (`self.PlayerSettingsSave`)))
  (bind _output_get (set `self.HasSaveFile` _returnvalue))
  (if _output_get
    (`self.LoadGame`)
    (`self.SaveGame`)
    (else
      (`self.CharacterSelect`)
      (`self.SaveGame`))))

(fn `Create_GameLift_Session`
  ;[0.1329 0.1912 0.2705] Create GameLift Session
  (`self.InitGameLift` :!enabledstate Disabled)
  (`self.StartGameSession` :!enabledstate Disabled))

(fn `DebugPrintMicSampling`
  (params (data :type "Array of Byte"))
  (locals (samples :type "Array of Byte"))
  (if (`KismetArrayLibrary.Array_IsNotEmpty` data)
    (bind _output_get (set `local.samples` data))
    (`KismetSystemLibrary.PrintString` (`KismetStringLibrary.Concat_StrStr` "bp received data from mic " (`KismetStringLibrary.Conv_IntToString` (`KismetArrayLibrary.Array_Length` _output_get))))))

(fn `DisableVolumeIndication`
  (`|ExecutionSequence`
    (:`then_0`
      (bind _rtcengine_eventhandle (`self.RtcEngine_EventHandle`)
        (:`then`
          (clear `IRtcEngineEventHandler.OnAudioVolumeIndication` _rtcengine_eventhandle))
        (:`else`)))))

(fn `EnableVolumeIndication`
  (params (BindEvent :type "Delegate (by ref)"))
  (`|ExecutionSequence`
    (:`then_0`
      (bind _rtcengine_eventhandle (`self.RtcEngine_EventHandle`)
        (:`then`
          (add `IRtcEngineEventHandler.OnAudioVolumeIndication` _rtcengine_eventhandle (`local.BindEvent`)))
        (:`else`)))
    (:`then_1`
      (bind _rtcengine_ref (`self.RtcEngine_Ref`)
        (:`then`
          (`AgoraRtcEngine.EnableAudioVolumeIndication` _rtcengine_ref 50 3 true))
        (:`else`)))))

(fn `FinishPixelStreaming`
  (bind _returnvalue (`Actor.GetComponentByClass` (`GameplayStatics.GetPlayerController` 0) null))
  (`/Engine/EditorBlueprintResources/StandardMacros.IsValid` _returnvalue
    (:`Is Valid`
      (`ActorComponent.K2_DestroyComponent` _returnvalue)
      (bind _pactor (`self.GetPixelStreamingActor` :!enabledstate Disabled))
      (`/Engine/EditorBlueprintResources/StandardMacros.IsValid` _pactor :!enabledstate Disabled
        (:`Is Valid`
          (`Actor.K2_DestroyActor` _pactor :!enabledstate Disabled))))))

(fn `InitSpatialVoice`
  (bind _localspatial (`self.LocalSpatial`))
  (bind _returnvalue (`AgoraRtcEngine.QueryInterface` (`self.RtcEngine_Ref`) "AGORA_IID_LOCAL_SPATIAL_AUDIO"))
  (bind _asilocal_spatial_audio_engine (cast `ILocalSpatialAudioEngine` _returnvalue))
  (bind _output_get (set `self.LocalSpatial` _asilocal_spatial_audio_engine))
  (`|VariableSetRef` (stale _config) (make `LocalSpatialAudioConfig` (`self.RtcEngine_Ref`)))
  (bind _config (`ILocalSpatialAudioEngine.Initialize` _output_get))
  (`ILocalSpatialAudioEngine.SetAudioRecvRange` _localspatial 20000.0)
  (`ILocalSpatialAudioEngine.SetDistanceUnit` _localspatial 0.01))

(fn `InitVoice`
  (bind _returnvalue (`GameplayStatics.GetPlayerController` 0))
  (`self.RtcEngine_Ref`
    (:`then`)
    (:`else`
      (bind _returnvalue_2 (`|GenericCreateObject` _returnvalue "/Script/AgoraPlugin.IRtcEngineEventHandler"))
      (bind _output_get (set `self.RtcEngine_EventHandle` _returnvalue_2))
      (bind _returnvalue_3 (`|GenericCreateObject` _returnvalue "/Script/AgoraPlugin.AgoraRtcEngine"))
      (bind _output_get_2 (set `self.RtcEngine_Ref` _returnvalue_3))
      (`AgoraRtcEngine.Initialize` _output_get_2 (make `RtcEngineContext` "13b44aa785094489a54fb06ee22d45c5" _output_get 0 "" "CHANNEL_PROFILE_COMMUNICATION" "AUDIO_SCENARIO_DEFAULT" false "HIGH"))
      (`AgoraRtcEngine.SetChannelProfile` (`self.RtcEngine_Ref`) "CHANNEL_PROFILE_LIVE_BROADCASTING")
      (`AgoraRtcEngine.SetClientRole` (`self.RtcEngine_Ref`) "CLIENT_ROLE_BROADCASTER")
      (`|ExecutionSequence`
        (:`then_0`
          (bind _returnvalue_4 (`AgoraRtcEngine.QueryInterface` (`self.RtcEngine_Ref`) "AGORA_IID_AUDIO_DEVICE_MANAGER"))
          (bind _asiaudio_device_manager (cast `IAudioDeviceManager` _returnvalue_4))
          (set `self.AudioDeviceManager` _asiaudio_device_manager))
        (:`then_1`
          (bind _returnvalue_5 (`GameplayStatics.LoadGameFromSlot` "DisplayMenu"))
          (bind _assave_display_menu (cast `/Game/XHUD/DisplayMenu/Save_DisplayMenu` _returnvalue_5))
          (`self.MuteVoice` (not (`/Game/XHUD/DisplayMenu/Save_DisplayMenu.IsMic_On` _assave_display_menu))))))))

(fn `JoinMatchServer`
  (params (GameSessionID :type String))
  (set `self.Gamesession_ID` GameSessionID)
  (set `self.IsJoinMatchServer` true)
  (`self.OpenLevel` "61.34.111.112"))

(fn `JoinVoiceChannel`
  (params (channelId :type String))
  (returns (Success :type Boolean))
  (bind _rtcengine_ref (`self.RtcEngine_Ref`)
    (:`then`
      (bind _returnvalue (`AgoraRtcEngine.JoinChannel` _rtcengine_ref "" "" (`KismetStringLibrary.Conv_StringToInt64` (`self.UserID`)) (make `ChannelMediaOptions` "AGORA_NULL_VALUE")))
      (return (== _returnvalue 0)))
    (:`else`)))

(fn `LeaveVoiceChannel`
  (bind _rtcengine_ref (`self.RtcEngine_Ref`)
    (:`then`
      (`AgoraRtcEngine.LeaveChannel` _rtcengine_ref (make `LeaveChannelOptions` "AGORA_NULL_VALUE")))
    (:`else`)))

(fn `LoadGame`
  (bind _returnvalue (`GameplayStatics.LoadGameFromSlot` (`self.PlayerSettingsSave`)))
  (bind _asbp_player_save_game_mp (cast `/Game/Multiplayer/Blueprints/BP_PlayerSaveGameMP` _returnvalue))
  (`|VariableSetRef` (`self.PlayerSettings`) (`/Game/Multiplayer/Blueprints/BP_PlayerSaveGameMP.S_PlayerInfo` _asbp_player_save_game_mp)))

(fn `LoginFailed`
  (set `self.UserID` ""))

(fn `MuteVoice`
  (params (mute :type Boolean))
  (returns (Success :type Boolean))
  (bind _rtcengine_ref (`self.RtcEngine_Ref`)
    (:`then`
      (set `self.IsMicMute` (`local.mute`))
      (bind _returnvalue (`AgoraRtcEngine.MuteLocalAudioStream` _rtcengine_ref (`local.mute`)))
      (return (== _returnvalue 0)))
    (:`else`)))

(fn `NetErrorToString`
  (params (FailureType :type "ENetworkFailure Enum" :default "NetDriverAlreadyExists"))
  (returns (OutString :type String))
  (return (`KismetStringLibrary.Concat_StrStr` "Error " (`|GetEnumeratorNameAsString` FailureType))))

(fn `NextLevel`
  (returns (Output_Get :type Integer))
  (bind _flobbylevellist_list_levelname (break `/Game/Map/FLobbyLevelList` (make `/Game/Map/FLobbyLevelList` _)))
  (bind _output_get (set `self.LobbyLevelNum` (mod (+ (`self.LobbyLevelNum`) 1) (`KismetArrayLibrary.Array_Length` _flobbylevellist_list_levelname))))
  (return _output_get))

(fn `OnResponsePlayerState`
  (params (PersonalState :type "/Game/XHUD/Profile/FPlayer_NameTag Structure"))
  (set `self.PersonalState` PersonalState))

(fn `OpenLobby`
  (`self.OpenLevel` "LoadingLevel"))

(fn `ReleaseVoice`
  (bind _rtcengine_ref (`self.RtcEngine_Ref`)
    (:`then`
      (`AgoraRtcEngine.LeaveChannel` _rtcengine_ref (make `LeaveChannelOptions` "AGORA_NULL_VALUE"))
      (`AgoraRtcEngine.UnregisterEventHandler` _rtcengine_ref (`self.RtcEngine_EventHandle`))
      (`AgoraRtcEngine.Release` _rtcengine_ref true)
      (set `self.RtcEngine_EventHandle` null)
      (set `self.RtcEngine_Ref` null))
    (:`else`)))

(fn `SaveGame`
  (bind _playersavegameref (`self.PlayerSaveGameRef`))
  (`self.PlayerSaveGameRef`
    (:`then`
      _)
    (:`else`
      (bind _returnvalue (`GameplayStatics.CreateSaveGameObject` "/Game/Multiplayer/Blueprints/BP_PlayerSaveGameMP.BP_PlayerSaveGameMP_C"))
      (set `self.PlayerSaveGameRef` _returnvalue)))
  (set `/Game/Multiplayer/Blueprints/BP_PlayerSaveGameMP.S_PlayerInfo` (`self.PlayerSettings`) _playersavegameref)
  (`GameplayStatics.SaveGameToSlot` _playersavegameref (`self.PlayerSettingsSave`)))

(fn `Set_WebView_SecretKey`
  (params (SecretKey :type String))
  (set `self.SecretKey` SecretKey))

(fn `SetDefaultAudioDevice`
  (locals (LocalRecordingDevices :type "IAudioDeviceCollection Object Reference") (LocalPlaybackDevices :type "IAudioDeviceCollection Object Reference"))
  (`self.AudioDeviceManager`
    (:`then`
      (`|ExecutionSequence`
        (:`then_0`
          (bind _returnvalue (`IAudioDeviceManager.EnumerateRecordingDevices` (`self.AudioDeviceManager`)))
          (set `local.LocalRecordingDevices` _returnvalue)
          (bind _returnvalue_2 (`IAudioDeviceCollection.GetCount` (`local.LocalRecordingDevices`)))
          (for _index (range (+ _returnvalue_2 1))
            (bind (_devicename _deviceid) (`IAudioDeviceCollection.GetDevice` (`local.LocalRecordingDevices`) _index))
            (if (`KismetStringLibrary.Contains` _devicename "Oculus Virtual Audio Device")
              (set `self.Mic_DeviceId` _deviceid)
              (`IAudioDeviceManager.SetRecordingDevice` (`self.AudioDeviceManager`) (`self.Mic_DeviceId`))
              (break))))
        (:`then_1`
          (bind _returnvalue_3 (`IAudioDeviceManager.EnumeratePlaybackDevices` (`self.AudioDeviceManager`)))
          (set `local.LocalPlaybackDevices` _returnvalue_3)
          (bind _returnvalue_4 (`IAudioDeviceCollection.GetCount` (`local.LocalPlaybackDevices`)))
          (for _index_2 (range (+ _returnvalue_4 1))
            (bind (_devicename_2 _deviceid_2) (`IAudioDeviceCollection.GetDevice` (`local.LocalPlaybackDevices`) _index_2))
            (if (`KismetStringLibrary.Contains` _devicename_2 "Oculus Virtual Audio Device")
              (set `self.Speaker_DeviceId` _deviceid_2)
              (`IAudioDeviceManager.SetPlaybackDevice` (`self.AudioDeviceManager`) (`self.Speaker_DeviceId`))
              (break))))))
    (:`else`)))

(fn `SetHostData`
  (params (IsHost :type Boolean) (GameID :type String) (UserCount :type Integer) (GameType :type String) (MapName :type String) (InMatchingGame :type Boolean))
  (if IsHost
    (set `self.isHost` IsHost)
    (set `self.Game_ID` GameID)
    (set `self.UserCount` UserCount)
    (set `self.MapName` MapName)
    (set `self.In Matching Game` InMatchingGame)
    (set `self.IsJoinMatchServer` false)
    (if (`self.IsDemo`)
      (bind _asbp_socket_io_demo (cast `/Game/Multiplayer/Demo/BP_SocketIO_Demo` (`/Game/Multiplayer/Blueprints/BP_GatePlayerController.SocketIoRef` (`/Game/Multiplayer/Blueprints/GateVRFunctionLibrary.GetGateController`))))
      (`/Game/Multiplayer/Demo/BP_SocketIO_Demo.Demo_Send_SessionID` _asbp_socket_io_demo "LocalDedicated")
      (elif (`self.In Matching Game`)
        (bind _asbp_socket_io_random_chat (cast `` (`/Game/Multiplayer/Blueprints/BP_GatePlayerController.SocketIoRef` (`/Game/Multiplayer/Blueprints/GateVRFunctionLibrary.GetGateController`) :!enabledstate Disabled) :!enabledstate Disabled))
        (`self.ue-matching-response-game-session` _asbp_socket_io_random_chat "TEST" :!enabledstate Disabled)
        (else
          (`/Game/Multiplayer/BP_SocketIO.Send_Game_FleetID` (`/Game/Multiplayer/Blueprints/BP_GatePlayerController.SocketIoRef` (`/Game/Multiplayer/Blueprints/GateVRFunctionLibrary.GetGateController`)) "LocalDedicated"))))
    (else
      (set `self.isHost` false))))

(fn `SetPlayerData`
  (params (IsHost :type Boolean) (IsinGame :type Boolean) (UserCount :type Integer) (GameID :type String) (FleetID :type String) (GameType :type String) (IsTest :type Boolean))
  (set `self.isHost` (`local.IsHost`))
  (set `self.isInGame` (`local.IsinGame`))
  (set `self.UserCount` (`local.UserCount`))
  (set `self.Game_ID` (`local.GameID`))
  (set `self.VoiceChannel` (`local.GameID`))
  (set `self.Gamesession_ID` (`local.FleetID`))
  (set `self.Game_Type` (`local.GameType`))
  (set `self.IsJoinMatchServer` false)
  (if IsTest
    (`self.OpenLevel` "61.34.111.112:7778")
    (else
      (`self.OpenLevel` "61.34.111.112"))))

(fn `SetVoiceEffect`
  (params (Effect :type Byte :default 0))
  (bind _rtcengine_ref (`self.RtcEngine_Ref`)
    (:`then`
      (`AgoraRtcEngine.SetVoiceConversionPreset` _rtcengine_ref (make `ENUMWRAP_VOICE_CONVERSION_PRESET` "VOICE_CONVERSION_OFF")))
    (:`else`)))

(fn `SpawnGateGameLift`
  (returns (GameLiftActor :type "Object Object Reference"))
  (`self.GateGameLiftRef`
    (:`then`)
    (:`else`
      (bind _returnvalue (`|SpawnActorFromClass` null (`KismetMathLibrary.MakeTransform` (0.0 0.0 0.0)) "Undefined" "OverrideRootScale" null null :!enabledstate Disabled))
      (set `self.GateGameLiftRef` null _returnvalue :!enabledstate Disabled)
      (return (`.GateGameLiftRef` (`self.GateGameLiftRef` :!enabledstate Disabled))))))

(fn `SpawnPixelStreamer`
  (`|SpawnActorFromClass` null (`KismetMathLibrary.MakeTransform` (0.0 0.0 0.0)) "Undefined" "OverrideRootScale" null null :!enabledstate Disabled))

(fn `Start_GameLift_Player`
  ;[0.1329 0.1912 0.2705] Start GameLift Player
  (`self.InitGameLift` :!enabledstate Disabled)
  (`self.Start_GameLift_Player_BindEvent` :!enabledstate Disabled)
  (`self.StartPlayer` :!enabledstate Disabled))

(fn `Start_GameLift_Player_BindEvent`
  (bind (_gategameliftref _gategameliftref_2) (`self.GateGameLiftRef` :!enabledstate Disabled)
    (:`then`
      (add `self.OnCreatePlayerSessionSuccess` _gategameliftref_2 (`|CreateDelegate` :!event `ReleaseVoice`) :!enabledstate Disabled))
    (:`else`)))

(fn `Start_GameLift_Session`
  ;[0.1198 1 0] Demo
  (if (`self.IsDemo` :!enabledstate Disabled)
    (bind _asbp_socket_io_demo (cast `/Game/Multiplayer/Demo/BP_SocketIO_Demo` (`/Game/Multiplayer/Blueprints/BP_GatePlayerController.SocketIoRef` (`/Game/Multiplayer/Blueprints/GateVRFunctionLibrary.GetGateController` :!enabledstate Disabled) :!enabledstate Disabled) :!enabledstate Disabled))
    (bind _gamelift (`self.InitGameLift` :!enabledstate Disabled))
    (set `self.GateGameLiftRef` null _gamelift :!enabledstate Disabled)
    (add `self.OnCreateGameSessionSuccess` _gamelift (`|CreateDelegate` _asbp_socket_io_demo :!event `Demo_Send_SessionID`) :!enabledstate Disabled)
    (`self.StartGameSession` :!enabledstate Disabled)
    (else
      ;[0.1329 0.1912 0.2705] Touring GameLift Session
      (`self.InitGameLift` :!enabledstate Disabled)
      (`self.BindEventOnCreateGameSession` :!enabledstate Disabled)
      (`self.StartGameSession` :!enabledstate Disabled))))

(fn `ToggleVoiceEcho`
  (params (Enable :type Boolean))
  (bind _rtcengine_ref (`self.RtcEngine_Ref`)
    (:`then`
      (`AgoraRtcEngine.SetAudioEffectPreset` _rtcengine_ref (select `bool` Enable :`false` (make `ENUMWRAP_AUDIO_EFFECT_PRESET` "AUDIO_EFFECT_OFF") :`true` (make `ENUMWRAP_AUDIO_EFFECT_PRESET` "ROOM_ACOUSTICS_VOCAL_CONCERT"))))
    (:`else`)))

(fn `TravelErrorToString`
  (params (FailureType :type "ETravelFailure Enum" :default "NoLevel"))
  (returns (OutString :type String))
  (return (`KismetStringLibrary.Concat_StrStr` "Error " (`|GetEnumeratorNameAsString` FailureType))))

(fn `TryLogin`
  (if (not (`self.IsLogin`))
    (set `self.IsLogin` true)))

(fn `UpdateRemoteLocation`
  (params (RemotePlayerPosition :type "Vector Structure") (RemotePlayerForward :type "Vector Structure") (RemotePlayerUid :type String))
  (`self.LocalSpatial`
    (:`then`
      (`|VariableSetRef` (stale _posinfo) (make `RemoteVoicePositionInfo` (`local.RemotePlayerPosition`) (`local.RemotePlayerForward`)))
      (bind _posinfo (`ILocalSpatialAudioEngine.UpdateRemotePosition` (`self.LocalSpatial`) (`KismetStringLibrary.Conv_StringToInt64` (`local.RemotePlayerUid`)))))
    (:`else`)))

(fn `UpdateSelfLocation`
  (bind _localspatial (`self.LocalSpatial`)
    (:`then`
      (bind _asbp_gate_character_vr (cast `/Game/Multiplayer/Characters/FBIK/BP_GateCharacter_VR` (`Controller.K2_GetPawn` (`GameplayStatics.GetPlayerController` 0))))
      (bind _camera (`/Game/Multiplayer/Characters/FBIK/BP_GateCharacter_VR.Camera` _asbp_gate_character_vr))
      (`ILocalSpatialAudioEngine.UpdateSelfPosition` _localspatial (`SceneComponent.K2_GetComponentLocation` _camera) (`SceneComponent.GetForwardVector` _camera) (`SceneComponent.GetRightVector` _camera) (`SceneComponent.GetUpVector` _camera)))
    (:`else`)))