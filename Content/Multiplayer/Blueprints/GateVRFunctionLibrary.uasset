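; Blueprint function library for the GateVR multiplayer game, giving shared static helpers to its Blueprints.
; Typed getters return the game instance, game mode, player state and local controller, which the laser-toggle and announcement helpers forward to.
; Other helpers pick a random lobby or untagged PlayerStart, map keys to levels with a fallback, test view and range, and sort actors by distance.
; String utilities substitute commands and indexed data tokens and build zero-padded timestamps.
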(fn `Announce`
  (params (Event :type "/Game/Multiplayer/Blueprints/Announcer/FAnnounceData Structure"))
  (`/Game/Multiplayer/Blueprints/BP_GatePlayerController.Announce_Server` (`self.GetGateController` null) Event))

(fn `AnnounceLocal`
  (params (Name :type String))
  (bind _asbp_gate_player_controller (cast `/Game/Multiplayer/Blueprints/BP_GatePlayerController` (`GameplayStatics.GetPlayerController` null)))
  (`/Game/Multiplayer/Blueprints/BP_GatePlayerController.Announce_Func` _asbp_gate_player_controller (make `/Game/Multiplayer/Blueprints/Announcer/FAnnounceData` :`Name` Name :`Team` (`/Game/Multiplayer/Blueprints/BP_GatePlayerController.Index_Team` _asbp_gate_player_controller) :`Instigator` _asbp_gate_player_controller)))

(fn `GetGateController`
  (returns (Controller :type "/Game/Multiplayer/Blueprints/BP_GatePlayerController Object Reference"))
  (bind _asbp_gate_player_controller (cast `/Game/Multiplayer/Blueprints/BP_GatePlayerController` (`GameplayStatics.GetPlayerController` null))
    (:`then`
      (return _asbp_gate_player_controller))
    (:`CastFailed`
      (return null))))

(fn `GetGateGamemode`
  (returns (Gamemode :type "/Game/Multiplayer/Blueprints/BP_GateGameMode Object Reference") (Success :type Boolean))
  (bind _asbp_gate_game_mode (cast `/Game/Multiplayer/Blueprints/BP_GateGameMode` (`GameplayStatics.GetGameMode` null))
    (:`then`
      (return _asbp_gate_game_mode true))
    (:`CastFailed`
      (return null false))))

(fn `GetGateInstance`
  (returns (Instance :type "/Game/Multiplayer/Blueprints/BP_GateGameInstance Object Reference"))
  (bind _returnvalue (`GameplayStatics.GetGameInstance` null))
  (`/Engine/EditorBlueprintResources/StandardMacros.IsValid` _returnvalue
    (:`Is Valid`
      (bind _asbp_gate_game_instance (cast `/Game/Multiplayer/Blueprints/BP_GateGameInstance` _returnvalue)
        (:`then`
          (return _asbp_gate_game_instance))
        (:`CastFailed`
          _)))
    (:`Is Not Valid`
      _))
  (return null))

(fn `GetGatePlayerStateByCharacter`
  (params (Character :type "Character Object Reference"))
  (returns (PlayerState :type "/Game/Multiplayer/Blueprints/BG_GatevrPlayerStateMP Object Reference") (Success :type Boolean))
  (bind _returnvalue (`Pawn.GetController` Character))
  (`/Engine/EditorBlueprintResources/StandardMacros.IsValid` _returnvalue
    (:`Is Valid`
      (bind _asbg_gatevr_player_state_mp (cast `/Game/Multiplayer/Blueprints/BG_GatevrPlayerStateMP` (`Controller.PlayerState` _returnvalue))
        (:`then`
          (return _asbg_gatevr_player_state_mp true))
        (:`CastFailed`
          (return null false))))
    (:`Is Not Valid`
      (return null false))))

(fn `GetGateRespawnPoint`
  (returns (Point :type "PlayerStart Object Reference"))
  (locals (Points :type "Array of PlayerStart Object Reference"))
  (bind _points (`local.Points`))
  (bind _outactors (`GameplayStatics.GetAllActorsOfClass` null "/Script/Engine.PlayerStart"))
  (for _array_element _outactors
    (bind _playerstarttag (`PlayerStart.PlayerStartTag` _array_element))
    (if (or (== _playerstarttag "None") (== _playerstarttag "None") (== _playerstarttag "Lobby"))
      (`KismetArrayLibrary.Array_Add` (`local.Points`) _array_element)))
  (return (`|GetArrayItem` _points (`KismetMathLibrary.RandomInteger` (`KismetArrayLibrary.Array_Length` _points)))))

(fn `GetGateStateByController`
  (params (Controller :type "Controller Object Reference"))
  (returns (PlayerState :type "/Game/Multiplayer/Blueprints/BG_GatevrPlayerStateMP Object Reference") (Success :type Boolean))
  (`/Engine/EditorBlueprintResources/StandardMacros.IsValid` Controller
    (:`Is Valid`
      (bind _asbg_gatevr_player_state_mp (cast `/Game/Multiplayer/Blueprints/BG_GatevrPlayerStateMP` (`Controller.PlayerState` Controller))
        (:`then`
          (return _asbg_gatevr_player_state_mp true))
        (:`CastFailed`
          (return null false))))
    (:`Is Not Valid`
      (return null false))))

(fn `GetNowTimeToString`
  (params (ShowTime :type Boolean) (GetFromUTC :type Boolean))
  (returns (Result :type String))
  (bind (_year _month _day _hour _minute _second _millisecond) (`KismetMathLibrary.BreakDateTime` (`KismetMathLibrary.UtcNow`)))
  (bind (_year_2 _month_2 _day_2 _hour_2 _minute_2 _second_2 _millisecond_2) (`KismetMathLibrary.BreakDateTime` (`KismetMathLibrary.Now`)))
  (bind _returnvalue (`KismetStringLibrary.Conv_IntToString` _month))
  (bind _returnvalue_2 (`KismetStringLibrary.Conv_IntToString` _day))
  (bind _returnvalue_3 (`KismetStringLibrary.Conv_IntToString` _hour))
  (bind _returnvalue_4 (`KismetStringLibrary.Conv_IntToString` _minute))
  (bind _returnvalue_5 (`KismetStringLibrary.Conv_IntToString` _second))
  (bind _returnvalue_6 (`KismetStringLibrary.Conv_IntToString` _month_2))
  (bind _returnvalue_7 (`KismetStringLibrary.Conv_IntToString` _day_2))
  (bind _returnvalue_8 (`KismetStringLibrary.Conv_IntToString` _hour_2))
  (bind _returnvalue_9 (`KismetStringLibrary.Conv_IntToString` _minute_2))
  (bind _returnvalue_10 (`KismetStringLibrary.Conv_IntToString` _second_2))
  (bind _returnvalue_11 (`KismetStringLibrary.GetSubstring` (`KismetStringLibrary.Conv_IntToString` _year) 2 4))
  (bind _returnvalue_12 (`KismetStringLibrary.GetSubstring` (`KismetStringLibrary.Conv_IntToString` _year_2) 2 4))
  (bind _returnvalue_13 (select `int` (`KismetStringLibrary.Len` _returnvalue) :`0` _returnvalue :`1` (`KismetStringLibrary.Concat_StrStr` "0" _returnvalue) :`2` _returnvalue))
  (bind _returnvalue_14 (select `int` (`KismetStringLibrary.Len` _returnvalue_6) :`0` _returnvalue_6 :`1` (`KismetStringLibrary.Concat_StrStr` "0" _returnvalue_6) :`2` _returnvalue_6))
  (bind _returnvalue_15 (select `int` (`KismetStringLibrary.Len` _returnvalue_7) :`0` _returnvalue_7 :`1` (`KismetStringLibrary.Concat_StrStr` "0" _returnvalue_7) :`2` _returnvalue_7))
  (bind _returnvalue_16 (select `int` (`KismetStringLibrary.Len` _returnvalue_2) :`0` _returnvalue_2 :`1` (`KismetStringLibrary.Concat_StrStr` "0" _returnvalue_2) :`2` _returnvalue_2))
  (if GetFromUTC
    (if ShowTime
      (return (`KismetStringLibrary.Concat_StrStr` _returnvalue_11 "-" _returnvalue_13 "-" _returnvalue_16 " " (select `int` (`KismetStringLibrary.Len` _returnvalue_3) :`0` _returnvalue_3 :`1` (`KismetStringLibrary.Concat_StrStr` "0" _returnvalue_3) :`2` _returnvalue_3) "." (select `int` (`KismetStringLibrary.Len` _returnvalue_4) :`0` _returnvalue_4 :`1` (`KismetStringLibrary.Concat_StrStr` "0" _returnvalue_4) :`2` _returnvalue_4) "." (select `int` (`KismetStringLibrary.Len` _returnvalue_5) :`0` _returnvalue_5 :`1` (`KismetStringLibrary.Concat_StrStr` "0" _returnvalue_5) :`2` _returnvalue_5) "."))
      (else
        (return (`KismetStringLibrary.Concat_StrStr` _returnvalue_11 "-" _returnvalue_13 "-" _returnvalue_16))))
    (elif ShowTime
      (return (`KismetStringLibrary.Concat_StrStr` _returnvalue_12 "-" _returnvalue_14 "-" _returnvalue_15 " " (select `int` (`KismetStringLibrary.Len` _returnvalue_8) :`0` _returnvalue_8 :`1` (`KismetStringLibrary.Concat_StrStr` "0" _returnvalue_8) :`2` _returnvalue_8) "." (select `int` (`KismetStringLibrary.Len` _returnvalue_9) :`0` _returnvalue_9 :`1` (`KismetStringLibrary.Concat_StrStr` "0" _returnvalue_9) :`2` _returnvalue_9) "." (select `int` (`KismetStringLibrary.Len` _returnvalue_10) :`0` _returnvalue_10 :`1` (`KismetStringLibrary.Concat_StrStr` "0" _returnvalue_10) :`2` _returnvalue_10) "."))
      (else
        (return (`KismetStringLibrary.Concat_StrStr` _returnvalue_12 "-" _returnvalue_14 "-" _returnvalue_15))))))

(fn `IsTargetInLocalView`
  (params (Target :type "SceneComponent Object Reference") (ViewAngle :type "Float (double-precision)" :default 30.0))
  (returns (InLocalView :type Boolean))
  (bind _returnvalue (`GameplayStatics.GetPlayerCameraManager` null))
  (bind _viewangle (`local.ViewAngle`))
  (bind (_returnvalue_roll _returnvalue_pitch _returnvalue_yaw) (`KismetMathLibrary.BreakRotator` (`KismetMathLibrary.NormalizedDeltaRotator` (`KismetMathLibrary.MakeRotFromX` (`KismetMathLibrary.Normal` (- (`SceneComponent.K2_GetComponentLocation` Target) (`PlayerCameraManager.GetCameraLocation` _returnvalue)))) (`PlayerCameraManager.GetCameraRotation` _returnvalue))))
  (`/Engine/EditorBlueprintResources/StandardMacros.IsValid` Target
    (:`Is Valid`
      (return (and (<= (`KismetMathLibrary.Abs` _returnvalue_pitch) _viewangle) (<= (`KismetMathLibrary.Abs` _returnvalue_yaw) _viewangle))))
    (:`Is Not Valid`
      (return false))))

(fn `IsTargetInRange`
  (params (Actor :type "SceneComponent Object Reference") (Target :type "Vector Structure") (Maximum :type "Float (double-precision)"))
  (returns (InRange :type Boolean))
  (`/Engine/EditorBlueprintResources/StandardMacros.IsValid` Actor
    (:`Is Valid`
      (return (<= (`KismetMathLibrary.VSizeXY` (- (`SceneComponent.K2_GetComponentLocation` Actor) Target)) Maximum)))
    (:`Is Not Valid`
      (return false))))

(fn `ReplaceCommand`
  (params (Original :type String) (Command :type String) (Replace :type String))
  (returns (Result :type String))
  (locals (Target :type "Array of String"))
  (bind _command (`local.Command`))
  (bind _command_2 (`local.Command`))
  (bind _output_get (set `local.Target` (`KismetStringLibrary.ParseIntoArray` Original)))
  (for (_array_element _array_index) _output_get
    (if (`KismetStringLibrary.Contains` _array_element _command)
      (`KismetArrayLibrary.Array_Set` (`local.Target`) _array_index (`KismetStringLibrary.Concat_StrStr` (`local.Replace`) (`.RightS` (`KismetStringLibrary.Split` _array_element (`KismetStringLibrary.Mid` _command (`KismetStringLibrary.FindSubstring` _array_element _command_2) (`KismetStringLibrary.Len` _command_2))))))))
  (return (`KismetStringLibrary.JoinStringArray` (`local.Target`))))

(fn `ReplaceData`
  (params (Original :type String) (Data :type "Array of String"))
  (returns (Result :type String))
  (locals (Target :type "Array of String") (Source :type String))
  (bind _data (`local.Data`))
  (bind _returnvalue (`KismetStringLibrary.FindSubstring` (`local.Source`) "{data:"))
  (bind _returnvalue_2 (`KismetStringLibrary.Mid` (`local.Source`) _returnvalue 8))
  (bind _returnvalue_3 (`KismetStringLibrary.Conv_StringToInt` (`KismetStringLibrary.Right` _returnvalue_2 2)))
  (if (`KismetStringLibrary.Contains` Original "{data:")
    (bind _output_get (set `local.Target` (`KismetStringLibrary.ParseIntoArray` Original)))
    (for (_array_element _array_index) _output_get
      (set `local.Source` _array_element)
      (if (`KismetStringLibrary.Contains` (`local.Source`) "{data:")
        (`KismetArrayLibrary.Array_Set` (`local.Target`) _array_index (`KismetStringLibrary.Concat_StrStr` (`KismetStringLibrary.Left` (`local.Source`) _returnvalue) (`KismetMathLibrary.SelectString` (`|GetArrayItem` _data _returnvalue_3) "?" (`KismetArrayLibrary.Array_IsValidIndex` _data _returnvalue_3)) (`.RightS` (`KismetStringLibrary.Split` (`local.Source`) _returnvalue_2))))))
    (return (`KismetStringLibrary.JoinStringArray` (`local.Target`)))
    (else
      (return (`local.Original`)))))

(fn `SelectLevel`
  (params (Key :type "String (by ref)"))
  (returns (ReturnValue :type String))
  (locals (MapMatch :type "Map of String to String"))
  (bind (_value _returnvalue) (`BlueprintMapLibrary.Map_Find` (`local.MapMatch`) Key))
  (bind _returnvalue_2 (`KismetMathLibrary.SelectString` _value "B5_001_A_06_P" _returnvalue))
  (`KismetSystemLibrary.PrintString` null _returnvalue_2 false)
  (return _returnvalue_2))

(fn `SortActorsClosest`
  (params (Actors :type "Array of Actor Object Reference") (Target :type "Vector Structure"))
  (returns (Result :type "Array of Actor Object Reference"))
  (locals (ToSwap :type "Actor Object Reference"))
  (bind _returnvalue (`KismetArrayLibrary.Array_LastIndex` Actors))
  (bind _actors (`local.Actors`))
  (bind _actors_2 (`local.Actors`))
  (if (> _returnvalue 1)
    (for _index (range 1 (+ _returnvalue 1))
      (for _index_2 (range (+ _returnvalue 1))
        (if (< (`KismetMathLibrary.VSize` (- (`Actor.K2_GetActorLocation` (`|GetArrayItem` (`local.Actors`) _index)) (`local.Target`))) (`KismetMathLibrary.VSize` (- (`Actor.K2_GetActorLocation` (`|GetArrayItem` (`local.Actors`) _index_2)) (`local.Target`))))
          (set `local.ToSwap` (`|GetArrayItem` _actors _index))
          (`KismetArrayLibrary.Array_Set` _actors_2 _index (`|GetArrayItem` _actors _index_2))
          (`KismetArrayLibrary.Array_Set` _actors_2 _index_2 (`local.ToSwap`))))))
  (return (`local.Actors`)))

(fn `ToggleLaser`
  (params (IsOn :type Boolean :default true) (Hand :type "/Game/Multiplayer/Blueprints/EHandSelection Enum" :default "NewEnumerator0") (AttachTo :type "SceneComponent Object Reference") (OwningMotionController :type "MotionControllerComponent Object Reference"))
  (bind _controller (`self.GetGateController` null))
  (bind _owningmotioncontroller (`local.OwningMotionController`))
  (bind _attachto (`local.AttachTo`))
  (if (`local.IsOn`)
    (if (`|EnumEquality` (`local.Hand`) "NewEnumerator2")
      (`/Game/Multiplayer/Blueprints/BP_GatePlayerController.ToggleLaser` _controller false _attachto _owningmotioncontroller)
      (`/Game/Multiplayer/Blueprints/BP_GatePlayerController.ToggleLaser` _controller true _attachto _owningmotioncontroller)
      (else
        (`/Game/Multiplayer/Blueprints/BP_GatePlayerController.ToggleLaser` (`self.GetGateController` null) (`|EnumEquality` (`local.Hand`) "NewEnumerator1") (`local.AttachTo`) (`local.OwningMotionController`))))
    (else
      (`/Game/Multiplayer/Blueprints/BP_GatePlayerController.DeleteLaser` (`self.GetGateController` null)))))