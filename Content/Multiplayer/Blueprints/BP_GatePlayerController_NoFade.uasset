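; Player controller for the VR login gate that, on BeginPlay, spawns a stereo login HUD or, if already logged in, a character-select web view.
; HUDs appear in front of the pawn using yaw only.
; Socket.IO events are bound for sign-in, login results and level travel, and the parent's level-load start, webview toggle and laser deletion are overridden empty.
; Holding right menu over three seconds while logged in opens a test level.
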(event `self.ReceiveBeginPlay`
  (`parent.ReceiveBeginPlay`)
  (`self.SpawnLoginUI`))

(event `EnhancedInput|/Game/VRTemplate/Input/Actions/IA_Menu_Toggle_Right`
  (params (ActionValue :type Boolean) (ElapsedSeconds :type "Float (double-precision)") (TriggeredSeconds :type "Float (double-precision)") (InputAction :type "InputAction Object Reference" :default "/Game/VRTemplate/Input/Actions/IA_Menu_Toggle_Right.IA_Menu_Toggle_Right"))
  (bind _instance (`/Game/Multiplayer/Blueprints/GateVRFunctionLibrary.GetGateInstance`))
  (:`Triggered`
    (if (> TriggeredSeconds 3.0)
      (if (`/Game/Multiplayer/Blueprints/BP_GateGameInstance.IsLogin` _instance)
        (`/Game/Multiplayer/Blueprints/BP_GateGameInstance.OpenLevel` _instance "Test_A3_002_A_08_P")))))

(fn `DeleteLaser`)

(fn `OpenLobbyLevel`
  (`/Game/Multiplayer/Blueprints/BP_GateGameInstance.OpenLevel` (`/Game/Multiplayer/Blueprints/GateVRFunctionLibrary.GetGateInstance`) "A5_001_A_00_P"))

(fn `PlayLoginResultSound`
  (params (IsSuccess :type Boolean))
  (`|ExecutionSequence`
    (:`then_0`
      (if (`local.IsSuccess`)
        (clear `/Game/Multiplayer/BP_SocketIO.CallOnPlayLoginResultSound` (`self.SocketIoRef`))))
    (:`then_1`
      (`GameplayStatics.PlaySound2D` (select `bool` (`local.IsSuccess`) :`true` "/Game/Sounds/Effect_Sound/Button/Cue_Button_02.Cue_Button_02" :!type "SoundBase Object Reference") 1.0 1.0 0.0 "/Game/Sounds/Effect_Sound/HUD/Concurrency_HUD.Concurrency_HUD" null))))

(fn `Socket_BindEvent`
  (`parent.Socket_BindEvent`)
  (add `/Game/Multiplayer/BP_SocketIO.OnSignedInSuccessfully` (`self.SocketIoRef`) (`|CreateDelegate` :!event `OpenLobbyLevel`))
  (if (not (`/Game/Multiplayer/Blueprints/BP_GateGameInstance.IsLogin` (`/Game/Multiplayer/Blueprints/GateVRFunctionLibrary.GetGateInstance`)))
    (add `/Game/Multiplayer/BP_SocketIO.CallOnPlayLoginResultSound` (`self.SocketIoRef`) (`|CreateDelegate` :!event `PlayLoginResultSound`))))

(fn `SpawnCharSelectHUD`
  (bind _returnvalue (`GameplayStatics.GetPlayerPawn` 0))
  (bind (_returnvalue_roll _returnvalue_pitch _returnvalue_yaw) (`KismetMathLibrary.BreakRotator` (`self.K2_GetActorRotation` _returnvalue)))
  (bind _returnvalue_2 (`KismetMathLibrary.MakeRotator` 0.0 0.0 _returnvalue_yaw))
  (`self.HUD_CharSelect`
    (:`then`)
    (:`else`
      (bind _returnvalue_3 (`|SpawnActorFromClass` "/Game/XHUD/BP_StereoWebViewHUD.BP_StereoWebViewHUD_C" (`KismetMathLibrary.MakeTransform` (+ (`self.K2_GetActorLocation` _returnvalue) (* (`KismetMathLibrary.GetForwardVector` _returnvalue_2) 220.0) (* (`KismetMathLibrary.GetUpVector` _returnvalue_2) 135.0)) _returnvalue_2) "AlwaysSpawn" "OverrideRootScale" null true "https://dev.app.gatevr.com/characters" null))
      (set `self.HUD_CharSelect` _returnvalue_3)
      (bind _socketioref (`self.SocketIoRef`)
        (:`then`
          (add `/Game/Multiplayer/BP_SocketIO.OnLevelTravel` _socketioref (`|CreateDelegate` (`self.HUD_CharSelect`) :!event `DoDestroy`))
          (`/Game/XHUD/BP_StereoWebViewHUD.LoadURL` (`self.HUD_CharSelect`)))
        (:`else`)))))

(fn `SpawnLoginHUD`
  (bind _returnvalue (`GameplayStatics.GetPlayerPawn` 0))
  (bind (_returnvalue_roll _returnvalue_pitch _returnvalue_yaw) (`KismetMathLibrary.BreakRotator` (`self.K2_GetActorRotation` _returnvalue)))
  (bind _returnvalue_2 (`KismetMathLibrary.MakeRotator` 0.0 0.0 _returnvalue_yaw))
  (`self.HUD_Login`
    (:`then`)
    (:`else`
      (bind _returnvalue_3 (`|SpawnActorFromClass` "/Game/XHUD/BP_StereoLoginHUD.BP_StereoLoginHUD_C" (`KismetMathLibrary.MakeTransform` (+ (`self.K2_GetActorLocation` _returnvalue) (* (`KismetMathLibrary.GetForwardVector` _returnvalue_2) 180.0) (* (`KismetMathLibrary.GetUpVector` _returnvalue_2) 135.0)) _returnvalue_2) "AlwaysSpawn" "OverrideRootScale" null null))
      (set `self.HUD_Login` _returnvalue_3)
      (bind _socketioref (`self.SocketIoRef`)
        (:`then`
          (add `/Game/Multiplayer/BP_SocketIO.OnLevelTravel` _socketioref (`|CreateDelegate` (`self.HUD_Login`) :!event `DoDestroy`))
          (add `/Game/Multiplayer/BP_SocketIO.OnLoginFailed` _socketioref (`|CreateDelegate` (`self.HUD_Login`) :!event `LoginFailed`))
          (add `/Game/Multiplayer/BP_SocketIO.OnResponseSecretKey` _socketioref (`|CreateDelegate` (`self.HUD_Login`) :!event `TryLoginWeb`)))
        (:`else`)))))

(fn `SpawnLoginUI`
  (if (`/Game/Multiplayer/Blueprints/BP_GateGameInstance.IsLogin` (`/Game/Multiplayer/Blueprints/GateVRFunctionLibrary.GetGateInstance`))
    (`self.SpawnCharSelectHUD`)
    (else
      (`self.SpawnLoginHUD`))))

(fn `StartLevelLoad`)

(fn `Toggle_Webview_HUD`
  (params (IsSetURL :type Boolean) (SetURL :type String)))

(fn `UserConstructionScript`
  (`parent.UserConstructionScript`))