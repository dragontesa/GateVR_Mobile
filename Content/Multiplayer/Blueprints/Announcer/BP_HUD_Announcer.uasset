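; BP_HUD_Announcer is a HUD announcer actor that shows announcement and notice widgets on stereo layers.
; A looping timer started at BeginPlay appears to retry Initialize until both widget render targets are valid, then binds them as layer textures and stops.
; Announce sends timed text to WBP_Announcer and plays a 2D sound, while Notice forwards events to WBP_Notice.
; DoDestroy clears both layer textures, then destroys the actor after a short delay.
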(event `self.ReceiveBeginPlay`
  (bind _returnvalue (`KismetSystemLibrary.K2_SetTimerDelegate` (`|CreateDelegate` :!event `Initialize`) 0.1 true))
  (set `self.Timer_Init` _returnvalue))

(event `DoDestroy`
  (`StereoLayerComponent.SetTexture` (`self.StereoLayer_Sub`) null)
  (`StereoLayerComponent.SetTexture` (`self.StereoLayer_Notice`) null)
  (`KismetSystemLibrary.Delay` 0.5)
  (`self.K2_DestroyActor`))

(fn `Announce`
  (params (Text :type String) (Time :type "Float (double-precision)") (SFX :type "SoundBase Object Reference"))
  (bind _aswbp_announcer (cast `/Game/Multiplayer/Blueprints/Announcer/WBP_Announcer` (`WidgetComponent.GetWidget` (`self.Widget_Sub`))))
  (`/Game/Multiplayer/Blueprints/Announcer/WBP_Announcer.Announce` _aswbp_announcer (`KismetTextLibrary.Conv_StringToText` (`local.Text`)) (`local.Time`))
  (`GameplayStatics.PlaySound2D` (`local.SFX`) 1.0 1.0 0.0 null null))

(fn `Initialize`
  (bind _returnvalue (`WidgetComponent.GetRenderTarget` (`self.Widget_Notice`)))
  (bind _returnvalue_2 (`WidgetComponent.GetRenderTarget` (`self.Widget_Sub`)))
  (if (and (`KismetSystemLibrary.IsValid` _returnvalue_2) (`KismetSystemLibrary.IsValid` _returnvalue))
    (`StereoLayerComponent.SetTexture` (`self.StereoLayer_Sub`) _returnvalue_2)
    (`StereoLayerComponent.SetTexture` (`self.StereoLayer_Notice`) _returnvalue)
    (`KismetSystemLibrary.K2_ClearAndInvalidateTimerHandle` (`self.Timer_Init`))))

(fn `Notice`
  (params (Event :type String))
  (bind _aswbp_notice (cast `/Game/Multiplayer/Blueprints/Announcer/WBP_Notice` (`WidgetComponent.GetWidget` (`self.Widget_Notice`))))
  (`/Game/Multiplayer/Blueprints/Announcer/WBP_Notice.Notice` _aswbp_notice Event))

(fn `UserConstructionScript`)