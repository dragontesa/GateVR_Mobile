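; Player controller component that updates VR character clothing, makeup and presets in multiplayer.
; On the local controller it binds to Socket.IO item changes and relays them through Server and All events; the user-info binding for character updates is disconnected.
; Underscore-delimited codes are parsed into part, type and name, then classes are found through the Asset Registry under /Game/ItemData, loaded synchronously and applied to the character.
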(event `self.ReceiveBeginPlay`
  (`KismetSystemLibrary.Delay` 1.0)
  (bind _asbp_gate_player_controller (cast `/Game/Multiplayer/Blueprints/BP_GatePlayerController` (`self.GetOwner`)))
  (if (`Controller.IsLocalPlayerController` _asbp_gate_player_controller)
    (bind _socketioref (`/Game/Multiplayer/Blueprints/BP_GatePlayerController.SocketIoRef` _asbp_gate_player_controller)
      (:`then`
        (add `/Game/Multiplayer/BP_SocketIO.ItemChanged` _socketioref (delegate `ItemUpdate_Local`)))
      (:`else`))))

(event `CharacterUpdate_Local`
  (params (CharacterCode :type String) (Parts :type "/Game/Multiplayer/Blueprints/CharParts/FPartsInfo Structure"))
  ;[0 0 0] Character
  (bind _asbp_gate_player_controller (cast `/Game/Multiplayer/Blueprints/BP_GatePlayerController` (`self.GetOwner`)))
  (bind _asbp_gate_character_vr (cast `/Game/Multiplayer/Characters/FBIK/BP_GateCharacter_VR` (`Controller.K2_GetPawn` _asbp_gate_player_controller)))
  (`self.CharacterUpdate_Server` _asbp_gate_character_vr CharacterCode Parts))

(event `ItemUpdate_Local`
  (params (ItemCode :type String) (IsWear :type Boolean))
  ;[0 0 0] Item
  (bind _asbp_gate_player_controller (cast `/Game/Multiplayer/Blueprints/BP_GatePlayerController` (`self.GetOwner`)))
  (bind _asbp_gate_character_vr (cast `/Game/Multiplayer/Characters/FBIK/BP_GateCharacter_VR` (`Controller.K2_GetPawn` _asbp_gate_player_controller)))
  (`self.ItemUpdate_Server` _asbp_gate_character_vr ItemCode))

(event `ItemUpdate_Server`
  (params (Character :type "/Game/Multiplayer/Characters/FBIK/BP_GateCharacter_VR Object Reference") (ItemCode :type String))
  ;[0 0 0] Item
  (`self.ItemUpdate_All` Character ItemCode))

(event `CharacterUpdate_Server`
  (params (Character :type "/Game/Multiplayer/Characters/BP_GateCharacter_Base Object Reference") (Code :type String) (Parts :type "/Game/Multiplayer/Blueprints/CharParts/FPartsInfo Structure"))
  ;[0 0 0] Character
  (`self.CharacterUpdate_All` Character Code Parts))

(event `ItemUpdate_All`
  (params (Character :type "/Game/Multiplayer/Characters/FBIK/BP_GateCharacter_VR Object Reference") (Code :type String))
  ;[0 0 0] Item
  (`self.ItemUpdate` Character Code))

(event `CharacterUpdate_All`
  (params (Character :type "/Game/Multiplayer/Characters/BP_GateCharacter_Base Object Reference") (Code :type String) (Parts :type "/Game/Multiplayer/Blueprints/CharParts/FPartsInfo Structure"))
  ;[0 0 0] Character
  (bind _ascharacter_preset (castclass `/Game/ItemData/Base/CharacterPreset` (`self.LoadAssetClass` "Character" (`self.ParseCharacterCode` Code))))
  (`self.CharacterUpdate` Character _ascharacter_preset)
  (`self.PartsUpdate` Character Parts))

(fn `CharacterUpdate`
  (params (Character :type "/Game/Multiplayer/Characters/BP_GateCharacter_Base Object Reference") (Class :type "Object Class Reference"))
  (bind _ascharacter_preset (castclass `/Game/ItemData/Base/CharacterPreset` Class))
  (bind _character (`local.Character`)
    (:`then`
      (set `/Game/Multiplayer/Characters/BP_GateCharacter_Base.CharacterSetClass` _ascharacter_preset _character)
      (`/Game/Multiplayer/Characters/BP_GateCharacter_Base.UpdateCharacter` _character))
    (:`else`)))

(fn `ItemUpdate`
  (params (Character :type "/Game/Multiplayer/Characters/BP_GateCharacter_Base Object Reference") (Code :type String))
  (locals (AssetClass :type "Object Class Reference") (CodeArray :type "Array of String") (ItemName :type String) (ItemType :type String) (ItemPart :type String) (ClothClass :type "/Game/ItemData/Base/ClothSet Class Reference") (MakeupClass :type "/Game/ItemData/Base/MakeupSet Class Reference"))
  (bind (_part _type _name) (`self.ParseItemCode` (`local.Code`)))
  (`|ExecutionSequence`
    (:`then_0`
      (set `local.ItemPart` _part)
      (set `local.ItemType` _type)
      (set `local.ItemName` _name))
    (:`then_1`
      (bind _output_get (set `local.AssetClass` (`self.LoadAssetClass` (`local.ItemPart`) (`local.ItemName`))))
      (if (`KismetSystemLibrary.IsValidClass` _output_get)
        (switch `string` (`local.ItemPart`)
          (:`Cloth`
            (`self.UpdateItem_Cloth` (`local.Character`) (`local.AssetClass`) (`local.ItemType`)))
          (:`Makeup`
            (`self.UpdateItem_Makeup` (`local.Character`) (`local.AssetClass`) (`local.ItemType`))))))))

(fn `LoadAssetClass`
  (params (Part :type String) (Name :type String))
  (returns (Class :type "Object Class Reference"))
  (bind (_outassetdata _returnvalue) (`AssetRegistry.GetAssetsByPackageName` (`AssetRegistryHelpers.GetAssetRegistry`) (`KismetStringLibrary.Conv_StringToName` (`KismetStringLibrary.Replace` (`KismetStringLibrary.Concat_StrStr` "/Game/ItemData/" Part "/" Name) " ")) false true))
  (if _returnvalue
    (bind _returnvalue_2 (`KismetSystemLibrary.GetPathName` (`AssetRegistryHelpers.GetAsset` (`|GetArrayItem` _outassetdata))))
    (bind _returnvalue_3 (`KismetSystemLibrary.LoadClassAsset_Blocking` (`KismetSystemLibrary.Conv_SoftClassPathToSoftClassRef` (`KismetSystemLibrary.MakeSoftClassPath` (select `bool` (== (`KismetStringLibrary.Right` _returnvalue_2 2) "_C") :`false` (`KismetStringLibrary.Concat_StrStr` _returnvalue_2 "_C") :`true` _returnvalue_2)))))
    (return _returnvalue_3)
    (else
      (return null))))

(fn `ParseCharacterCode`
  (params (Code :type String))
  (returns (Name :type String))
  (locals (CodeArray :type "Array of String"))
  (set `local.CodeArray` (`KismetStringLibrary.ParseIntoArray` Code "_"))
  (return (`KismetStringLibrary.Concat_StrStr` "CharacterPreset_" (`BlueprintMapLibrary.Map_Find` (`self.CodeName_Gender`) (`|GetArrayItem` (`local.CodeArray`))) "_" (`|GetArrayItem` (`local.CodeArray`) 1))))

(fn `ParseItemCode`
  (params (Code :type String))
  (returns (Part :type String) (Type :type String) (Name :type String))
  (locals (CodeArray :type "Array of String") (ItemPart :type String) (ItemName :type String) (ItemType :type String))
  (`|ExecutionSequence`
    (:`then_0`
      (bind _output_get (set `local.CodeArray` (`KismetStringLibrary.ParseIntoArray` Code "_")))
      (switch `string` (`|GetArrayItem` _output_get)
        (:`P3`
          (set `local.ItemPart` "Cloth")
          (set `local.ItemName` (`KismetStringLibrary.Concat_StrStr` (`BlueprintMapLibrary.Map_Find` (`self.CodeName_Parts`) (`|GetArrayItem` (`local.CodeArray`))) "_" (`BlueprintMapLibrary.Map_Find` (`self.CodeName_Gender`) (`|GetArrayItem` (`local.CodeArray`) 1)) "_" (`BlueprintMapLibrary.Map_Find` (`self.CodeName_Body`) (`|GetArrayItem` (`local.CodeArray`) 2)) "_" (`BlueprintMapLibrary.Map_Find` (`self.CodeName_ClothType`) (`|GetArrayItem` (`local.CodeArray`) 3)) "_" (`|GetArrayItem` (`local.CodeArray`) 4) "_" (`|GetArrayItem` (`local.CodeArray`) 5)))
          (set `local.ItemType` (`BlueprintMapLibrary.Map_Find` (`self.CodeName_ClothType`) (`|GetArrayItem` (`local.CodeArray`) 3))))
        (:`P4`
          (set `local.ItemPart` "Makeup")
          (set `local.ItemName` (`KismetStringLibrary.Concat_StrStr` (`BlueprintMapLibrary.Map_Find` (`self.CodeName_Parts`) (`|GetArrayItem` (`local.CodeArray`))) "_" (`BlueprintMapLibrary.Map_Find` (`self.CodeName_Gender`) (`|GetArrayItem` (`local.CodeArray`) 1)) "_" (`BlueprintMapLibrary.Map_Find` (`self.CodeName_MakeupType`) (`|GetArrayItem` (`local.CodeArray`) 2)) "_" (`|GetArrayItem` (`local.CodeArray`) 3) "_" (`|GetArrayItem` (`local.CodeArray`) 4)))
          (set `local.ItemType` (`BlueprintMapLibrary.Map_Find` (`self.CodeName_MakeupType`) (`|GetArrayItem` (`local.CodeArray`) 2))))))
    (:`then_1`
      (return (`local.ItemPart`) (`local.ItemType`) (`local.ItemName`)))))

(fn `PartsUpdate`
  (params (Character :type "/Game/Multiplayer/Characters/BP_GateCharacter_Base Object Reference") (Parts :type "/Game/Multiplayer/Blueprints/CharParts/FPartsInfo Structure"))
  (bind _output_get (set `self.PartsInfo` Parts))
  (`self.ItemUpdate` (`local.Character`) (break `/Game/Multiplayer/Blueprints/CharParts/FPartsInfo` _output_get))
  (`self.ItemUpdate` (`local.Character`) (`.Lower_13_DC512B1143A6DAE176B088B268A8629B` (break `/Game/Multiplayer/Blueprints/CharParts/FPartsInfo` _output_get)))
  (`self.ItemUpdate` (`local.Character`) (`.Shoes_11_D8B7C2E34384EB474216F0A87363DD5A` (break `/Game/Multiplayer/Blueprints/CharParts/FPartsInfo` _output_get)))
  (`self.ItemUpdate` (`local.Character`) (`.Makeup_16_B018BD37494130F128B73C8CF5FD5ABB` (break `/Game/Multiplayer/Blueprints/CharParts/FPartsInfo` _output_get))))

(fn `UpdateItem_Cloth`
  (params (Character :type "/Game/Multiplayer/Characters/BP_GateCharacter_Base Object Reference") (Class :type "Object Class Reference") (Type :type String))
  (locals (ClothClass :type "/Game/ItemData/Base/ClothSet Class Reference"))
  (bind _ascloth_set (castclass `/Game/ItemData/Base/ClothSet` Class))
  (set `local.ClothClass` _ascloth_set)
  (switch `string` (`local.Type`)
    (:`UpIn`
      (`/Game/Multiplayer/Characters/BP_GateCharacter_Base.UpdateUpper` (`local.Character`) (`local.ClothClass`) :!label _label))
    (:`UpOut`
      (goto _label))
    (:`Set`
      (goto _label))
    (:`LowIn`
      (`/Game/Multiplayer/Characters/BP_GateCharacter_Base.UpdateLower` (`local.Character`) (`local.ClothClass`) :!label _label_2))
    (:`LowOut`
      (goto _label_2))
    (:`Shoes`
      (`/Game/Multiplayer/Characters/BP_GateCharacter_Base.UpdateShoes` (`local.Character`) (`local.ClothClass`)))))

(fn `UpdateItem_Makeup`
  (params (Character :type "/Game/Multiplayer/Characters/BP_GateCharacter_Base Object Reference") (Class :type "Object Class Reference") (Type :type String))
  (locals (MakeupClass :type "/Game/ItemData/Base/MakeupSet Class Reference"))
  (bind _asmakeup_set (castclass `/Game/ItemData/Base/MakeupSet` Class))
  (set `local.MakeupClass` _asmakeup_set)
  (switch `string` (`local.Type`)
    (:`Full`
      (`/Game/Multiplayer/Characters/BP_GateCharacter_Base.UpdateMakeup` (`local.Character`) (`local.MakeupClass`)))))

(fn `UserConstructionScript`)