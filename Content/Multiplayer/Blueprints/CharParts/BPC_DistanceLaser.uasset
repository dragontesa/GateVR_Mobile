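; VR motion-controller component that drives a laser pointer for UI clicks, actor interaction and distance grabbing in multiplayer.
; While on, tick favors widget hits, otherwise line-traces to update the LaserActor beam and cache grabbable actors not locked by another pointer.
; Trigger presses the widget pointer and sends interactions through server and multicast events.
; Grab functions lock the target, disable physics and fly it along a clamped arc toward the controller.
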(event `self.ReceiveBeginPlay`
  (`/Engine/EditorBlueprintResources/StandardMacros.IsValid` (`self.OwningMotionController`)
    (:`Is Valid`
      (`self.K2_AttachToComponent` self (`self.OwningMotionController`) "None" "KeepRelative" "KeepRelative" "KeepRelative" true)
      (`self.SetLaserBeam` false))))

(event `SetLaserBeam`
  (params (IsOn :type Boolean) (LaserActor_ref :type "/Game/Multiplayer/Blueprints/CharParts/BP_LaserActor Object Reference"))
  (bind _output_get (set `self.Is On` IsOn))
  (if _output_get
    (`/Engine/EditorBlueprintResources/StandardMacros.IsValid` LaserActor_ref
      (:`Is Valid`
        (bind _output_get_2 (set `self.LaserActor` LaserActor_ref))
        (`/Game/Multiplayer/Blueprints/CharParts/BP_LaserActor.AttachLaserComp` _output_get_2 (`self.OwningMotionController`))
        (`self.SetComponentTickEnabled` true)))
    (else
      (`self.SetComponentTickEnabled` false)
      (bind _laseractor (`self.LaserActor`)
        (:`then`
          (`/Game/Multiplayer/Blueprints/CharParts/BP_LaserActor.OffLaserBeam` _laseractor)
          (`Actor.K2_DestroyActor` _laseractor))
        (:`else`)))))

(event `self.ReceiveTick`
  (params (DeltaSeconds :type "Float (single-precision)"))
  (`self.UpdateLaser`))

(event `InteractionAction_Ser`
  (params (InteractActor :type "Actor Object Reference"))
  ;[1 1 1] Interaction Action
  (`self.InteractionAction_M` InteractActor))

(event `InteractionAction_M`
  (params (InteractActor :type "Actor Object Reference"))
  ;[1 1 1] Interaction Action
  (message `/Game/LevelDesign/Assets/Blueprints/BP_Interface_InteractionActor.InteractionAction` InteractActor null (0.0 0.0 0.0)))

(fn `EndFly`
  (bind _grabbleactorref (`self.GrabbleActorRef`)
    (:`then`
      (`PrimitiveComponent.SetSimulatePhysics` (`/Game/LevelDesign/Assets/Blueprints/BP_GrabActor_Base_MP.SM_Root` (`self.GrabbleActorRef`)) false)
      (bind _bpc_grabcomp_mp (`/Game/LevelDesign/Assets/Blueprints/BP_GrabActor_Base_MP.BPC_GrabComp_MP` _grabbleactorref))
      (bind _locklaserpointer (`/Game/LevelDesign/Assets/Blueprints/BPC_GrabComp_MP.LockLaserPointer` _bpc_grabcomp_mp)
        (:`then`
          (if (== _locklaserpointer self)
            (set `/Game/LevelDesign/Assets/Blueprints/BPC_GrabComp_MP.LockLaserPointer` null _bpc_grabcomp_mp)
            (`self.OnFinished`)))
        (:`else`
          _)))
    (:`else`
      _))
  (set `self.GrabbleActorRef` null))

(fn `Fly Grab Actor`
  (params (`Alpha XY` :type "Float (double-precision)") (`Alpha Z` :type "Float (double-precision)"))
  (bind _grabbleactorref (`self.GrabbleActorRef`)
    (:`then`
      (`Actor.K2_SetActorLocation` _grabbleactorref (`self.SetFlyPath` `Alpha XY` `Alpha Z` (`self.Impact Point`) (`self.Arc Apex Multiplier`) (`self.Arc Apex Max Z`)) false false))
    (:`else`)))

(fn `Get Interaction Actor`
  (returns (Isvalid :type Boolean) (`Last Hit Result Hit Actor` :type "Actor Object Reference"))
  (bind (_lasthitresult_bblockinghit _lasthitresult_binitialoverlap _lasthitresult_time _lasthitresult_distance _lasthitresult_location _lasthitresult_impactpoint _lasthitresult_normal _lasthitresult_impactnormal _lasthitresult_physmat _lasthitresult_hitactor) (`GameplayStatics.BreakHitResult` (`self.LastHitResult`)))
  (`self.GrabbleActorRef`
    (:`then`
      (return false null))
    (:`else`
      (`/Engine/EditorBlueprintResources/StandardMacros.IsValid` _lasthitresult_hitactor
        (:`Is Valid`
          (return true _lasthitresult_hitactor))
        (:`Is Not Valid`
          (return false null))))))

(fn `Grab Actor Locking`
  (bind _grabbleactorref (`self.GrabbleActorRef`)
    (:`then`
      (`self.SetComponentTickEnabled` false)
      (set `/Game/LevelDesign/Assets/Blueprints/BPC_GrabComp_MP.Lock` self (`/Game/LevelDesign/Assets/Blueprints/BP_GrabActor_Base_MP.BPC_GrabComp_MP` _grabbleactorref))
      (`PrimitiveComponent.SetSimulatePhysics` (`/Game/LevelDesign/Assets/Blueprints/BP_GrabActor_Base_MP.SM_Root` (`self.GrabbleActorRef`)) false))
    (:`else`)))

(fn `IsOverlapWidget`
  (returns (IsOverlap :type Boolean))
  (bind _widgetinteraction (`/Game/Multiplayer/Blueprints/CharParts/BP_LaserActor.WidgetInteraction` (`self.LaserActor`)))
  (return (or (`WidgetInteractionComponent.IsOverInteractableWidget` _widgetinteraction) (`WidgetInteractionComponent.IsOverFocusableWidget` _widgetinteraction))))

(fn `SetFlyPath`
  (params (`Alpha XY` :type "Float (double-precision)") (`Alpha Z` :type "Float (double-precision)") (Origin :type "Vector Structure") (`Arc Apex Multiplier` :type "Float (double-precision)") (`Arc Apex Max Z` :type "Float (double-precision)"))
  (returns (ReturnValue :type "Vector Structure"))
  (bind _returnvalue (`self.K2_GetComponentLocation` (`self.OwningMotionController`)))
  (return (`KismetMathLibrary.VLerp` Origin (+ _returnvalue (`KismetMathLibrary.MakeVector` 0.0 0.0 (`KismetMathLibrary.Lerp` 0.0 (`KismetMathLibrary.FClamp` (* (`KismetMathLibrary.Vector_Distance` Origin _returnvalue) (* `Arc Apex Multiplier` 0.1)) 0.0 `Arc Apex Max Z`) `Alpha Z`))) `Alpha XY`)))

(fn `TriggerRelease`
  (`WidgetInteractionComponent.ReleasePointerKey` (`/Game/Multiplayer/Blueprints/CharParts/BP_LaserActor.WidgetInteraction` (`self.LaserActor`)) "LeftMouseButton"))

(fn `TriggerStart`
  (bind _isvalid (`self.Get Interaction Actor`))
  (if _isvalid
    (`self.InteractionAction_Ser` null))
  (`WidgetInteractionComponent.PressPointerKey` (`/Game/Multiplayer/Blueprints/CharParts/BP_LaserActor.WidgetInteraction` (`self.LaserActor`)) "LeftMouseButton"))

(fn `UpdateLaser`
  (bind _owningmotioncontroller (`self.OwningMotionController`))
  (bind _returnvalue (`self.K2_GetComponentLocation` _owningmotioncontroller))
  (bind (_bblockinghit _binitialoverlap _time _distance _location _impactpoint _normal _impactnormal _physmat _hitactor) (`GameplayStatics.BreakHitResult` (`self.LastHitResult`)))
  (bind _returnvalue_2 (`Actor.GetComponentByClass` _hitactor "/Game/LevelDesign/Assets/Blueprints/BPC_GrabComp_MP.BPC_GrabComp_MP_C"))
  (bind _ownergrabactor (`/Game/LevelDesign/Assets/Blueprints/BPC_GrabComp_MP.OwnerGrabActor` _returnvalue_2))
  (bind _bpc_grabcomp_mp (`/Game/LevelDesign/Assets/Blueprints/BP_GrabActor_Base_MP.BPC_GrabComp_MP` _ownergrabactor))
  (if (`self.IsOverlapWidget`)
    ;[1 1 1] HitWidget
    (`/Game/Multiplayer/Blueprints/CharParts/BP_LaserActor.OnHitWidgetLaserBeam` (`self.LaserActor`))
    (else
      ;[1 1 1] HitIntaeraction Actor
      (bind (_outhit _returnvalue_3) (`KismetSystemLibrary.LineTraceSingle` _returnvalue (+ _returnvalue (* (`KismetMathLibrary.GetForwardVector` (`self.K2_GetComponentRotation` _owningmotioncontroller)) (`self.Interaction Distance`))) "TraceTypeQuery7" false (`|MakeArray` (`self.GetOwner` (`self.OwningMotionController`))) "None" true (struct :`B` 1.0 :`A` 1.0)))
      (set `self.LastHitResult` _outhit)
      (if _returnvalue_3
        (`|ExecutionSequence`
          (:`then_0`
            ;[0 0.06733 0.4531] If Gravity Grab Actor isnt already available, store to variable. If already available, update to the new traced item
            (`/Engine/EditorBlueprintResources/StandardMacros.IsValid` _returnvalue_2
              (:`Is Valid`
                (bind _locklaserpointer (`/Game/LevelDesign/Assets/Blueprints/BPC_GrabComp_MP.LockLaserPointer` _bpc_grabcomp_mp)
                  (:`then`
                    (if (== self _locklaserpointer)
                      (if true :!label _label
                        (set `self.GrabCompnentRef` _bpc_grabcomp_mp)
                        (bind _grabbleactorref (`self.GrabbleActorRef`)
                          (:`then`
                            (if (not (== _grabbleactorref _ownergrabactor))
                              (set `self.GrabbleActorRef` _ownergrabactor :!label _label_2)))
                          (:`else`
                            (goto _label_2)))
                        (set `self.Impact Point` _impactpoint))
                      (else
                        (set `self.GrabbleActorRef` null))))
                  (:`else`
                    (goto _label))))))
          (:`then_1`
            (`/Game/Multiplayer/Blueprints/CharParts/BP_LaserActor.OnHitInteractionActorLaserBeam` (`self.LaserActor`) (`self.LastHitResult`))))
        (else
          ;[1 1 1] Interaction Nothing
          (`|ExecutionSequence`
            (:`then_0`
              (`self.GrabbleActorRef`
                (:`then`
                  (set `self.GrabbleActorRef` null)
                  (set `self.GrabCompnentRef` null))
                (:`else`)))
            (:`then_1`
              (`/Game/Multiplayer/Blueprints/CharParts/BP_LaserActor.UpdateLaserBeam` (`self.LaserActor`) (`self.Interaction Distance`)))))))))