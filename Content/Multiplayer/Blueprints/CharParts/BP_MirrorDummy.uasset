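; BP_MirrorDummy is a modular character double that mirrors the player character's pose and carries a scene capture camera.
; Body follows the player's Body through leader pose on BeginPlay, while construction links the clothing and accessory parts to Body.
; SetScenePosition steps the capture through head, upper and body sockets, returning true once no further position remains.
; Construction also calls it, and SetSkeletalMseh is an empty stub.
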(event `self.ReceiveBeginPlay`
  (`SkinnedMeshComponent.SetLeaderPoseComponent` (`self.Body`) (`/Game/Multiplayer/Characters/FBIK/BP_GateCharacter_VR.Body` (`self.PlayerCharacter_Ref`)) false false))

(fn `SetScenePosition`
  (returns (IsDelete :type Boolean))
  (bind _scenecapturecomponent2d (`self.SceneCaptureComponent2D`))
  (bind _returnvalue (+ (`self.PositionNumber`) 1))
  (if (> _returnvalue 2)
    (return true)
    (else
      (bind _output_get (set `self.PositionNumber` (mod _returnvalue 3)))
      (`SceneComponent.K2_AttachToComponent` _scenecapturecomponent2d (`self.Body`) (select `int` _output_get :`0` "Socket_CameraPosition_Head" :`1` "Socket_CameraPosition_Upper" :`2` "Socket_CameraPosition_Body" :!type "Name") "KeepRelative" "KeepRelative" "KeepRelative" true)
      (`SceneComponent.K2_SetRelativeLocation` _scenecapturecomponent2d (0.0 0.0 0.0) false false)
      (return false))))

(fn `SetSkeletalMseh`)

(fn `UserConstructionScript`
  (`/Engine/EditorBlueprintResources/StandardMacros.IsValid` (`SkeletalMeshComponent.SkeletalMeshAsset` (`self.Face`)) ; Only create MIDs when there is a valid skeletal mesh is set \n(this prevents warnings in MH export)
    (:`Is Valid`
      (`SkinnedMeshComponent.SetLeaderPoseComponent` (`self.Feet`) (`self.Body`) false false)
      (`SkinnedMeshComponent.SetLeaderPoseComponent` (`self.Legs`) (`self.Body`) false false)
      (`SkinnedMeshComponent.SetLeaderPoseComponent` (`self.Torso`) (`self.Body`) false false)
      (`SkinnedMeshComponent.SetLeaderPoseComponent` (`self.Accessories1`) (`self.Body`) false false)
      (`SkinnedMeshComponent.SetLeaderPoseComponent` (`self.Accessories2`) (`self.Body`) false false)
      (`SkinnedMeshComponent.SetLeaderPoseComponent` (`self.Hat`) (`self.Body`) false false)
      (`self.SetScenePosition`))))