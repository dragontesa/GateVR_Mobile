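; Spatial voice component that feeds player positions to the Gate instance, apparently for positional voice chat in multiplayer VR.
; On non-dedicated instances with a local player controller, BeginPlay starts a fast looping timer, presumably driving UpdateLocation.
; UpdateLocation loops over all BP_GateCharacter_VR actors, updating self location if the Gate instance's UserID is empty.
; Otherwise it passes each character's camera position and forward vector as a remote location.
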(event `self.ReceiveBeginPlay`
  (if (`self.IsLocal`)
    (`KismetSystemLibrary.K2_SetTimerDelegate` (`|CreateDelegate` :!event `UpdateLocation`) 0.1 true)))

(fn `IsLocal`
  (returns (IsLocal :type Boolean))
  (bind _returnvalue (`GameplayStatics.GetPlayerController` 0))
  (if (`KismetSystemLibrary.IsDedicatedServer`)
    (return false)
    (else
      (`/Engine/EditorBlueprintResources/StandardMacros.IsValid` _returnvalue
        (:`Is Valid`
          (return (`Controller.IsLocalController` _returnvalue)))
        (:`Is Not Valid`
          (return false))))))

(fn `UpdateLocation`
  (bind _instance (`/Game/Multiplayer/Blueprints/GateVRFunctionLibrary.GetGateInstance`))
  (bind _outactors (`GameplayStatics.GetAllActorsOfClass` "/Game/Multiplayer/Characters/FBIK/BP_GateCharacter_VR.BP_GateCharacter_VR_C"))
  (for _array_element _outactors
    (if (`KismetStringLibrary.EqualEqual_StrStr` "" (`/Game/Multiplayer/Blueprints/BP_GateGameInstance.UserID` (`/Game/Multiplayer/Blueprints/GateVRFunctionLibrary.GetGateInstance`)))
      (`/Game/Multiplayer/Blueprints/BP_GateGameInstance.UpdateSelfLocation` _instance)
      (else
        (bind _camera (`/Game/Multiplayer/Characters/FBIK/BP_GateCharacter_VR.Camera` _array_element))
        (`/Game/Multiplayer/Blueprints/BP_GateGameInstance.UpdateRemoteLocation` _instance (`self.K2_GetComponentLocation` _camera) (`self.GetForwardVector` _camera) "")
        (`/Engine/EditorBlueprintResources/StandardMacros.DoOnce` false
          (:`Completed`
            (`KismetSystemLibrary.PrintString` "UpdateRemoteLocation" false)))))))