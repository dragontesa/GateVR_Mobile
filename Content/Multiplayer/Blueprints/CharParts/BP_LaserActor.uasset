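; BP_LaserActor is a laser pointer for character interaction, pairing a WidgetInteraction component with beam and end-point components that attach to a supplied parent.
; Externally called functions show the end point at a widget or actor hit, extend the beam to maximum distance without it, or switch both off.
; Beam length comes from setting world X scale directly to the distance in units.
; A setter assigns the widget pointer index, allowing separate pointers.
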(fn `AttachLaserComp`
  (params (Parent :type "SceneComponent Object Reference"))
  (`SceneComponent.K2_AttachToComponent` (`self.WidgetInteraction`) Parent "None" "KeepRelative" "KeepRelative" "KeepRelative" true)
  (`SceneComponent.K2_AttachToComponent` (`self.LaserBeam`) Parent "None" "KeepRelative" "KeepRelative" "KeepRelative" true)
  (`SceneComponent.K2_AttachToComponent` (`self.LaserBeamEndPoint`) Parent "None" "KeepRelative" "KeepRelative" "KeepRelative" true))

(fn `OffLaserBeam`
  (`SceneComponent.SetWorldScale3D` (`self.LaserBeam`) (0.0 0.0 0.0))
  (`SceneComponent.SetVisibility` (`self.LaserBeamEndPoint`) false false)
  (`SceneComponent.SetVisibility` (`self.LaserBeam`) false false))

(fn `OnHitInteractionActorLaserBeam`
  (params (Hit :type "HitResult Structure (by ref)"))
  (bind (_bblockinghit _binitialoverlap _time _distance _location _impactpoint) (`GameplayStatics.BreakHitResult` Hit))
  (`SceneComponent.SetVisibility` (`self.LaserBeamEndPoint`) true false)
  (`SceneComponent.K2_SetWorldLocation` (`self.LaserBeamEndPoint`) _impactpoint false false)
  (`SceneComponent.SetWorldScale3D` (`self.LaserBeam`) (`KismetMathLibrary.MakeVector` (`KismetMathLibrary.Vector_Distance` _impactpoint (`SceneComponent.K2_GetComponentLocation` (`self.LaserBeam`))) 0.5 0.5)))

(fn `OnHitWidgetLaserBeam`
  (bind (_returnvalue_bblockinghit _returnvalue_binitialoverlap _returnvalue_time _returnvalue_distance _returnvalue_location _returnvalue_impactpoint) (`GameplayStatics.BreakHitResult` (`WidgetInteractionComponent.GetLastHitResult` (`self.WidgetInteraction`))))
  ;[1 1 1] Interaction Widget
  (`SceneComponent.SetVisibility` (`self.LaserBeamEndPoint`) true false)
  (`SceneComponent.K2_SetWorldLocation` (`self.LaserBeamEndPoint`) _returnvalue_impactpoint false false)
  (`SceneComponent.SetWorldScale3D` (`self.LaserBeam`) (`KismetMathLibrary.MakeVector` (`KismetMathLibrary.Vector_Distance` _returnvalue_impactpoint (`SceneComponent.K2_GetComponentLocation` (`self.LaserBeam`))) 0.5 0.5)))

(fn `SetWidgetPointIndex`
  (params (`Pointer Index` :type Integer))
  (set `WidgetInteractionComponent.PointerIndex` `Pointer Index` (`self.WidgetInteraction`)))

(fn `UpdateLaserBeam`
  (params (MaxDistance :type "Float (double-precision)"))
  (`SceneComponent.SetWorldScale3D` (`self.LaserBeam`) (`KismetMathLibrary.MakeVector` MaxDistance 0.5 0.5))
  (`SceneComponent.SetVisibility` (`self.LaserBeamEndPoint`) false false))

(fn `UserConstructionScript`)