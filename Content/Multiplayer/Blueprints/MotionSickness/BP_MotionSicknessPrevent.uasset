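; BP_MotionSicknessPrevent is a VR comfort actor that fades a sphere material effect in while the player moves or turns.
; On construct it binds to the owning BP_GateCharacter_VR's move and turn inputs and attaches to player 0's camera manager.
; Each tick it interpolates the dynamic material's Alpha parameter from combined input magnitude, fading in faster than out.
; It destroys itself when that character is destroyed.
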(event `Construct`
  (bind _returnvalue (`PrimitiveComponent.CreateDynamicMaterialInstance` (`self.Sphere`) 0 "/Game/Multiplayer/Blueprints/MotionSickness/MI_MotionSicknessPrevent.MI_MotionSicknessPrevent" "None"))
  (set `self.MI_MotionSickness` _returnvalue)
  (bind _asbp_gate_character_vr (cast `/Game/Multiplayer/Characters/FBIK/BP_GateCharacter_VR` (`self.GetOwner`)))
  (add `/Game/Multiplayer/Characters/FBIK/BP_GateCharacter_VR.InputMoveForward` _asbp_gate_character_vr (delegate `MoveFoward`))
  (add `/Game/Multiplayer/Characters/FBIK/BP_GateCharacter_VR.InputMoveRight` _asbp_gate_character_vr (delegate `MoveRight`))
  (add `/Game/Multiplayer/Characters/FBIK/BP_GateCharacter_VR.InputTurn` _asbp_gate_character_vr (delegate `MoveTurn`))
  (add `self.OnDestroyed` _asbp_gate_character_vr (delegate `DestroyedParent`))
  (`self.K2_AttachToComponent` (`PlayerCameraManager.TransformComponent` (`GameplayStatics.GetPlayerCameraManager` 0)) "None" "SnapToTarget" "SnapToTarget" "KeepWorld"))

(event `MoveFoward`
  (params (ActionValue :type "Float (double-precision)"))
  (set `self.Foward` (`KismetMathLibrary.Abs` ActionValue)))

(event `DestroyedParent` :!signature `self.OnDestroyed`
  (params (DestroyedActor :type "Actor Object Reference"))
  (`self.K2_DestroyActor`))

(event `MoveRight`
  (params (ActionValue :type "Float (double-precision)"))
  (set `self.Right` (`KismetMathLibrary.Abs` ActionValue)))

(event `MoveTurn`
  (params (ActionValue :type "Float (double-precision)"))
  (set `self.Turn` (`KismetMathLibrary.Abs` ActionValue)))

(event `self.ReceiveTick`
  (params (DeltaSeconds :type "Float (single-precision)"))
  (bind _targetalpha (`self.TargetAlpha`))
  (bind _currentalpha (`self.CurrentAlpha`))
  (set `self.TargetAlpha` (`KismetMathLibrary.SelectFloat` 1.0 0.0 (> (+ (`self.Foward`) (`self.Right`) (`self.Turn`)) 0.1)))
  (bind _output_get (set `self.CurrentAlpha` (`KismetMathLibrary.FInterpTo_Constant` _currentalpha _targetalpha (`GameplayStatics.GetWorldDeltaSeconds`) (`KismetMathLibrary.SelectFloat` 3.0 1.0 (< _currentalpha _targetalpha)))))
  (`self.SetAlpha` _output_get))

(event `SetAlpha`
  (params (Value :type "Float (single-precision)"))
  (bind _mi_motionsickness (`self.MI_MotionSickness`)
    (:`then`
      (`MaterialInstanceDynamic.SetScalarParameterValue` _mi_motionsickness "Alpha" Value))
    (:`else`)))

(fn `UserConstructionScript`)