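; Debug multiplayer mode Blueprint that handles player respawning with the MP_Gate_DebugPC pawn class.
; RespawnPlayer destroys the controller's current pawn, if valid, then calls SpawnPawn.
; SpawnPawn spawns the class at a random spawn point, adjusting for collisions but always spawning.
; If the spawned actor is a Character, the controller possesses it and SpawnPersonalStateUI is called for that controller.
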(event `self.RespawnPlayer`
  (params (PlayerController :type "PlayerController Object Reference") (PlayerCharacter :type "Character Class Reference"))
  (bind _returnvalue (`Controller.K2_GetPawn` PlayerController))
  (`/Engine/EditorBlueprintResources/StandardMacros.IsValid` _returnvalue
    (:`Is Valid`
      (`self.K2_DestroyActor` _returnvalue))
    (:`Is Not Valid`
      _))
  (`self.SpawnPawn` PlayerController "/Game/Multiplayer/Characters/MP_Gate_DebugPC.MP_Gate_DebugPC_C"))

(fn `SpawnPawn`
  (params (Controller :type "PlayerController Object Reference") (Class :type "Actor Class Reference"))
  (bind (_returnvalue_location _returnvalue_rotation) (`KismetMathLibrary.BreakTransform` (`self.GetRandomSpawnPoint`)))
  (bind _returnvalue (`|SpawnActorFromClass` Class (`KismetMathLibrary.MakeTransform` _returnvalue_location _returnvalue_rotation) "AdjustIfPossibleButAlwaysSpawn" "SelectDefaultAtRuntime" null null))
  (bind _ascharacter (cast `Character` _returnvalue))
  (`Controller.Possess` Controller _ascharacter)
  (`self.SpawnPersonalStateUI` Controller))

(fn `UserConstructionScript`
  (`parent.UserConstructionScript`))