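; BP_RespawnCollision is a multiplayer trigger volume that recovers VR characters and physics items that enter its box.
; On overlap, only the server (authority) runs the respawn logic, passing the actor to both respawn functions, which filter it by cast.
; Characters have movement stopped and are teleported without fade to the gate respawn point's location and rotation.
; Physics items teleport back to their last position.
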(event `self.Box.OnComponentBeginOverlap`
  (params (OverlappedComponent :type "PrimitiveComponent Object Reference") (OtherActor :type "Actor Object Reference") (OtherComp :type "PrimitiveComponent Object Reference") (OtherBodyIndex :type Integer) (bFromSweep :type Boolean) (SweepResult :type "HitResult Structure (by ref)"))
  (`/Engine/EditorBlueprintResources/ActorMacros.Switch Has Authority`
    (:`Authority`
      (`self.RespawnPlayer` OtherActor)
      (`self.RespawnItem` OtherActor))))

(fn `RespawnItem`
  (params (Actor :type "Object Object Reference"))
  (bind _asbp_physics_item_base (cast `/Game/Animations/VRFBIK/Item/BP_PhysicsItem_Base` Actor))
  (`/Game/Animations/VRFBIK/Item/BP_PhysicsItem_Base.TeleportToLastPosition` _asbp_physics_item_base))

(fn `RespawnPlayer`
  (params (Actor :type "Object Object Reference"))
  (bind (_returnvalue_location _returnvalue_rotation) (`KismetMathLibrary.BreakTransform` (`self.GetTransform` (`/Game/Multiplayer/Blueprints/GateVRFunctionLibrary.GetGateRespawnPoint`))))
  (bind _asbp_gate_character_vr (cast `/Game/Multiplayer/Characters/FBIK/BP_GateCharacter_VR` Actor))
  (`MovementComponent.StopMovementImmediately` (`Character.CharacterMovement` _asbp_gate_character_vr))
  (`/Game/Multiplayer/Characters/FBIK/BP_GateCharacter_VR.Teleportation_All` :`self` _asbp_gate_character_vr :`NewLocation` _returnvalue_location :`NewRotation` _returnvalue_rotation :`IsFade` false))

(fn `UserConstructionScript`)