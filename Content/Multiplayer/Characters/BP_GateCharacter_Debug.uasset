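; Debug variant of the multiplayer VR Gate character, playable with mouse and keyboard by disabling the HMD and removing face tracking.
; Each tick pins both motion controllers ahead of the camera to fake hand poses and updates the teleport trace.
; Mouse buttons drive trigger, laser and VRIK server grab for the Space-selected hand; keys handle teleport and calibration.
; Axis inputs look, turn and move, with movement exiting chairs when blocked.
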(event EventBeginPlay
  ;[1 1 1] Begin & Tick
  (|CallParentFunction)
  (Class|HeadMountedDisplayFunctionLibrary|EnableHMD false)
  (Components|DestroyComponent (Variables|Default|GetGateXRFaceTracking)))

(event EventTick
  (params (DeltaSeconds :type Float%20%28single-precision%29))
  ;[1 1 1] Begin & Tick
  (|CallParentFunction DeltaSeconds)
  (CallFunction|UpdateHandPose)
  (CallFunction|TeleportTrace))

(event Input|AxisEvents|InputAxisLookUp
  (params (AxisValue :type Float%20%28single-precision%29))
  ;[1 1 1] LookUp
  (Transformation|AddRelativeRotation (Variables|Default|GetCamera) (Math|Rotator|MakeRotator 0.0 (* AxisValue -1.0) 0.0) false false))

(event Input|AxisEvents|InputAxisMoveForward/Backward
  (params (AxisValue :type Float%20%28single-precision%29))
  (bind _returnvalue (Math|Float|Absolute(Float) AxisValue))
  (bind _deadzone_stick (Variables|Default|GetDeadZone_Stick))
  (bind _returnvalue_2 (> _returnvalue _deadzone_stick))
  ;[1 1 1] Input Move & Trun
  (if (Default|IsModeMoveBlocked (CallFunction|GetGateController))
    (if _returnvalue_2
      (bind _vrik (Variables|Default|GetVRIK)
        (:then
          (if (Variables|/Game/Animations/VRFBIK/V2/BP_VRIK_V2.BP_VRIK_V2_C|GetIsSittingChair _vrik)
            (Default|EscapeonChair _vrik)))
        (:else)))
    (else
      (bind _output_get (Variables|Default|SetMoveInput_Y (Math|Float|SelectFloat AxisValue 0.0 _returnvalue_2)))
      (Default|CallInputMoveForward _output_get))))

(event Input|AxisEvents|InputAxisMoveRight/Left
  (params (AxisValue :type Float%20%28single-precision%29))
  (bind _returnvalue (Math|Float|Absolute(Float) AxisValue))
  (bind _deadzone_stick (Variables|Default|GetDeadZone_Stick))
  (bind _returnvalue_2 (> _returnvalue _deadzone_stick))
  ;[1 1 1] Input Move & Trun
  (if (Default|IsModeMoveBlocked (CallFunction|GetGateController))
    (if _returnvalue_2
      (bind _vrik (Variables|Default|GetVRIK)
        (:then
          (if (Variables|/Game/Animations/VRFBIK/V2/BP_VRIK_V2.BP_VRIK_V2_C|GetIsSittingChair _vrik)
            (Default|EscapeonChair _vrik)))
        (:else)))
    (else
      (bind _output_get (Variables|Default|SetMoveInput_X (Math|Float|SelectFloat AxisValue 0.0 _returnvalue_2)))
      (Default|CallInputMoveRight _output_get))))

(event Input|AxisEvents|InputAxisTurnRight/LeftMouse
  (params (AxisValue :type Float%20%28single-precision%29))
  (bind _returnvalue (Math|Float|Absolute(Float) AxisValue))
  (bind _returnvalue_2 (> _returnvalue 0.0))
  (bind _returnvalue_3 (Math|Float|SelectFloat AxisValue 0.0 _returnvalue_2))
  ;[1 1 1] Input Move & Trun
  (if (not (Default|IsModeMoveBlocked (CallFunction|GetGateController)))
    (Pawn|Input|AddControllerYawInput _returnvalue_3)
    (Default|CallInputTurn _returnvalue_3)))

(event Input|MouseEvents|MouseWheelAxis
  (params (AxisValue :type Float%20%28single-precision%29))
  ;[1 1 1] Wheel - Relative Move
  (Transformation|AddRelativeLocation (Variables|Default|GetCamera) (* "1.000000,0.000000,0.000000" (* AxisValue 5.0)) false false))

(event Input|KeyboardEvents|DebugKeySpaceBar
  (params (Key :type Key%20Structure :default "None") (ActionValue :type Input%20Action%20Value%20Structure))
  ;[1 1 1] Space Bar - Swap Hand
  (:Pressed
    (bind _isa (Utilities|FlowControl|FlipFlop)
      (:A
        _)
      (:B
        _))
    (Variables|Default|SetIsLeft _isa)))

(event Input|KeyboardEvents|R
  (params (Key :type Key%20Structure :default "None"))
  ;[1 1 1] R - Calibration
  (:Pressed
    (CallFunction|Calibration)))

(event Input|MouseEvents|LeftMouseButton
  (params (Key :type Key%20Structure :default "None"))
  (bind _motioncontrollerr (Variables|Default|GetMotionControllerR))
  (bind _motioncontrollerl (Variables|Default|GetMotionControllerL))
  ;[1 1 1] Left Click - Trigger
  (:Pressed
    (if (Variables|Default|GetIsLeft)
      (bind _vrik (Variables|Default|GetVRIK)
        (:then
          (bind _grabactor_l (Variables|/Game/Animations/VRFBIK/V2/BP_VRIK_V2.BP_VRIK_V2_C|GetGrabActor_L _vrik)
            (:then
              (Class|BPIPhysicsItem|Trigger(Message) _grabactor_l _motioncontrollerl true))
            (:else
              (CallFunction|ToggleLaser true "NewEnumerator0" _motioncontrollerl _motioncontrollerl))))
        (:else))
      (else
        (bind _vrik_2 (Variables|Default|GetVRIK)
          (:then
            (bind _grabactor_r (Variables|/Game/Animations/VRFBIK/V2/BP_VRIK_V2.BP_VRIK_V2_C|GetGrabActor_R _vrik_2)
              (:then
                (Class|BPIPhysicsItem|Trigger(Message) _grabactor_r _motioncontrollerr true))
              (:else
                (CallFunction|ToggleLaser true "NewEnumerator1" _motioncontrollerr _motioncontrollerr))))
          (:else)))))
  (:Released
    (if (Variables|Default|GetIsLeft)
      (bind _vrik_3 (Variables|Default|GetVRIK)
        (:then
          (bind _grabactor_l_2 (Variables|/Game/Animations/VRFBIK/V2/BP_VRIK_V2.BP_VRIK_V2_C|GetGrabActor_L _vrik_3)
            (:then
              (Class|BPIPhysicsItem|Trigger(Message) _grabactor_l_2 (Variables|Default|GetMotionControllerL) false))
            (:else
              (bind _ref_leftlaser (Variables|/Game/Multiplayer/Blueprints/BP_GatePlayerController.BP_GatePlayerController_C|GetRef_LeftLaser (CallFunction|GetGateController))
                (:then
                  (Default|TriggerRelease _ref_leftlaser))
                (:else)))))
        (:else))
      (else
        (bind _vrik_4 (Variables|Default|GetVRIK)
          (:then
            (bind _grabactor_r_2 (Variables|/Game/Animations/VRFBIK/V2/BP_VRIK_V2.BP_VRIK_V2_C|GetGrabActor_R _vrik_4)
              (:then
                (Class|BPIPhysicsItem|Trigger(Message) _grabactor_r_2 (Variables|Default|GetMotionControllerR) false))
              (:else
                (bind _ref_rightlaser (Variables|/Game/Multiplayer/Blueprints/BP_GatePlayerController.BP_GatePlayerController_C|GetRef_RightLaser (CallFunction|GetGateController))
                  (:then
                    (Default|TriggerRelease _ref_rightlaser))
                  (:else)))))
          (:else))))))

(event Input|MouseEvents|RightMouseButton
  (params (Key :type Key%20Structure :default "None"))
  (bind _isleft (Variables|Default|GetIsLeft))
  ;[1 1 1] Right Click - Grab
  (:Pressed
    (bind _vrik (Variables|Default|GetVRIK)
      (:then
        (Default|TryGrabServer _vrik _isleft))
      (:else)))
  (:Released
    (bind _vrik_2 (Variables|Default|GetVRIK)
      (:then
        (Default|TryReleaseServer _vrik_2 _isleft))
      (:else))))

(event Input|KeyboardEvents|T
  (params (Key :type Key%20Structure :default "None"))
  (:Pressed
    (CallFunction|StartTeleportTrace))
  (:Released
    (CallFunction|EndTeleportTrace)))

(fn ConstructionScript
  (|CallParentFunction))

(fn UpdateHandPose
  (bind _camera (Variables|Default|GetCamera))
  (bind _motioncontrollerr (Variables|Default|GetMotionControllerR))
  (bind _camera_2 (Variables|Default|GetCamera))
  (bind _motioncontrollerl (Variables|Default|GetMotionControllerL))
  (bind _returnvalue (Transformation|GetWorldTransform _camera))
  (bind _returnvalue_2 (Transformation|GetWorldTransform _camera_2))
  (bind _returnvalue_3 (Math|Vector|GetRightVector (.rotation _returnvalue_2)))
  (bind _returnvalue_4 (Math|Vector|GetUpVector (.rotation _returnvalue_2)))
  (bind _returnvalue_5 (Math|Vector|GetForwardVector (.rotation _returnvalue_2)))
  (bind _returnvalue_6 (Math|Vector|GetForwardVector (.rotation _returnvalue)))
  (bind _returnvalue_7 (Math|Vector|GetRightVector (.rotation _returnvalue)))
  (bind _returnvalue_8 (Math|Vector|GetUpVector (.rotation _returnvalue)))
  (bind _returnvalue_9 (* _returnvalue_6 5e+01))
  (bind _returnvalue_10 (* _returnvalue_4 -1e+01))
  (bind _returnvalue_11 (* _returnvalue_3 -5.0))
  (bind _returnvalue_12 (* _returnvalue_5 5e+01))
  (bind _returnvalue_13 (* _returnvalue_7 5.0))
  (bind _returnvalue_14 (* _returnvalue_8 -1e+01))
  (bind _returnvalue_15 (+ (.location _returnvalue) _returnvalue_9 _returnvalue_13 _returnvalue_14))
  (bind _returnvalue_16 (+ (.location _returnvalue_2) _returnvalue_12 _returnvalue_11 _returnvalue_10))
  (Utilities|FlowControl|Sequence
    (:then_0
      (Transformation|SetWorldLocationAndRotation _motioncontrollerr _returnvalue_15 (Math|Rotator|FindLookatRotation _returnvalue_15 (+ (.location _returnvalue) (* (Math|Vector|GetForwardVector (.rotation _returnvalue)) 1e+03))) false false)
      (Transformation|AddRelativeRotation _motioncontrollerr "0, 0, 0" false false))
    (:then_1
      (Transformation|SetWorldLocationAndRotation _motioncontrollerl _returnvalue_16 (Math|Rotator|FindLookatRotation _returnvalue_16 (+ (.location _returnvalue_2) (* (Math|Vector|GetForwardVector (.rotation _returnvalue_2)) 1e+03))) false false)
      (Transformation|AddRelativeRotation _motioncontrollerl "0, 0, 0" false false))))

(fn UpdateFaceExpression)

(fn SendFaceExpression)

(fn InitFaceTracking)