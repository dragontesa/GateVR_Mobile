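; BP_GateCharacter_NPC is an NPC mannequin character that can be grabbed by a motion controller and turned in place.
; AttachActorComp stores the controller and its starting rotation, hides the gate controller's laser and starts a fast looping timer, which DetachActor undoes.
; SetActorRotate turns the actor by a yaw step scaled from the controller's yaw offset since the grab.
; UpdateBody derives IsMale from the body class's display name.
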(event `/Game/Multiplayer/Blueprints/CharParts/BP_Interface_AttachActor.DetachActor`
  (set `self.IsAttach` false)
  (set `self.MotionController` null)
  (`/Game/Multiplayer/Blueprints/BP_GatePlayerController.SetHiddenLaser` (`/Game/Multiplayer/Blueprints/GateVRFunctionLibrary.GetGateController`) false)
  (`KismetSystemLibrary.K2_ClearAndInvalidateTimerHandle` (`self.TimeHandle`)))

(fn `AttachActorComp`
  (params (Parent :type "SceneComponent Object Reference"))
  (returns (IsAttach :type Boolean) (AttachActor :type "Actor Object Reference"))
  (if (`self.IsAttach`)
    (return false null)
    (else
      (set `self.IsAttach` true)
      (bind _output_get (set `self.MotionController` (`local.Parent`)))
      (set `self.StartRotate` (`SceneComponent.RelativeRotation` _output_get))
      (bind _returnvalue (`KismetSystemLibrary.K2_SetTimerDelegate` (`|CreateDelegate` :!event `SetActorRotate`) 0.01 true))
      (set `self.TimeHandle` _returnvalue)
      (`/Game/Multiplayer/Blueprints/BP_GatePlayerController.SetHiddenLaser` (`/Game/Multiplayer/Blueprints/GateVRFunctionLibrary.GetGateController`) true)
      (return true self))))

(fn `SetActorRotate`
  (bind (_returnvalue_roll _returnvalue_pitch _returnvalue_yaw) (`KismetMathLibrary.BreakRotator` (`self.K2_GetActorRotation`)))
  (bind (_startrotate_roll _startrotate_pitch _startrotate_yaw) (`KismetMathLibrary.BreakRotator` (`self.StartRotate`)))
  (bind (_relativerotation_roll _relativerotation_pitch _relativerotation_yaw) (`KismetMathLibrary.BreakRotator` (`SceneComponent.RelativeRotation` (`self.MotionController`))))
  (`self.K2_SetActorRotation` (`KismetMathLibrary.MakeRotator` _returnvalue_roll _returnvalue_pitch (+ _returnvalue_yaw (`KismetMathLibrary.MapRangeUnclamped` (- _startrotate_yaw _relativerotation_yaw) -180.0 180.0 -5.0 5.0)))))

(fn `UpdateBody`
  (params (Class :type "/Game/ItemData/Base/BodySet Class Reference"))
  (`parent.UpdateBody` Class)
  (bind _class (`local.Class`)
    (:`then`
      (set `self.IsMale` (== (`|GetArrayItem` (`KismetStringLibrary.ParseIntoArray` (`KismetSystemLibrary.GetClassDisplayName` _class) "_") 1) "M")))
    (:`else`)))

(fn `UserConstructionScript`
  (`parent.UserConstructionScript`))