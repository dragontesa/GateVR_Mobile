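; Mobile VR variant of the multiplayer Gate character, adding a hand-gesture spawn shortcut on top of its parent's behavior.
; When the right thumb-up input has been triggered for over three seconds, it prints a message and spawns a preset female mannequin at the view point, lowered and yaw-aligned.
; An unconnected chain would spawn a copy of this character turned around and call its Calibration.
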(event `EnhancedInput|/Game/VRTemplate/Input/Actions/Hands/IA_Hand_ThumbUp_Right`
  (params (ActionValue :type Boolean) (ElapsedSeconds :type "Float (double-precision)") (TriggeredSeconds :type "Float (double-precision)") (InputAction :type "InputAction Object Reference" :default "/Game/VRTemplate/Input/Actions/Hands/IA_Hand_ThumbUp_Right.IA_Hand_ThumbUp_Right"))
  (bind (_location _rotation) (`Controller.GetPlayerViewPoint` (`/Game/Multiplayer/Blueprints/GateVRFunctionLibrary.GetGateController`)))
  (:`Triggered`
    (if (> TriggeredSeconds 3.0)
      (`KismetSystemLibrary.PrintString` "A Right Pressed" true true (struct :`R` 1.0 :`G` 0.089761 :`B` 0.583388 :`A` 1.0))
      (`|SpawnActorFromClass` "/Game/Multiplayer/Characters/Mannquin/BC_G_Mannequin_F_01.BC_G_Mannequin_F_01_C" (`KismetMathLibrary.MakeTransform` (`KismetMathLibrary.MakeVector` (.x _location) (.y _location) (+ (.z _location) -100.0)) (`KismetMathLibrary.MakeRotator` 0.0 0.0 (.yaw _rotation))) "Undefined" "MultiplyWithRoot" null "/Game/ItemData/Character/CharacterPreset_F_0.CharacterPreset_F_0_C" null))))

(event `self.ReceiveBeginPlay`
  (`parent.ReceiveBeginPlay`))

(fn `UserConstructionScript`
  (`parent.UserConstructionScript`))